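; Menu controller for an RTS that owns the front-end screens and switches between them.
; On BeginPlay it creates and stores the main menu and mission select widgets, shows the main menu and enables the mouse cursor.
; Navigation events take the previous widget, remove it and add the cached target screen to the viewport.
; The load/save event only removes the previous widget, with no replacement screen shown.
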(event Custom|ToMainMenu
  (params (PreviousUI :type Widget%20Object%20Reference))
  (Widget|RemovefromParent PreviousUI)
  (UserInterface|Viewport|AddtoViewport (Variables|Default|GetMainMenuUI) 0))

(event Custom|ToLoadSave
  (params (PreviousUI :type Widget%20Object%20Reference))
  (Widget|RemovefromParent PreviousUI))

(event Custom|ToMissionSelect
  (params (PreviousUI :type Widget%20Object%20Reference))
  (Widget|RemovefromParent PreviousUI)
  (UserInterface|Viewport|AddtoViewport (Variables|Default|GetMissionSelectUI) 0))

(event EventBeginPlay
  (Utilities|FlowControl|Sequence
    (:then_0
      (bind _returnvalue (UserInterface|CreateWidget "/Game/Blueprints/UserInterface/Menus/WBP_MainMenu.WBP_MainMenu_C"))
      (Variables|Default|SetMainMenuUI _returnvalue))
    (:then_1
      (bind _returnvalue_2 (UserInterface|CreateWidget "/Game/Blueprints/UserInterface/Menus/WBP_MissionSelect.WBP_MissionSelect_C"))
      (Variables|Default|SetMissionSelectUI _returnvalue_2))
    (:then_3
      (UserInterface|Viewport|AddtoViewport (Variables|Default|GetMainMenuUI) 0)
      (Variables|Default|SetbShowMouseCursor true))))

(event EventTick
  (params (DeltaSeconds :type Float%20%28single-precision%29)))

(fn ConstructionScript)