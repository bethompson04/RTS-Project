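; BP_AICommander is an AI commander actor that spawns squads and directs their movement.
; On BeginPlay it builds squads from DT_Squads rows, making the first unit leader, and caches the objective tracker.
; Tick runs FindMovement per squad, writing heard enemy locations to the leader's blackboard as move targets.
; The Extermination branch is an empty loop, the EQS query is unconnected, and a Delay sits inside the Tick loop.
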(event EventBeginPlay
  (CallFunction|SpawnSquads)
  (bind _returnvalue (Actor|GetActorOfClass "/Game/Levels/BP_ObjectiveTracker.BP_ObjectiveTracker_C"))
  (Utilities|IsValid _returnvalue
    (:Is%20Valid
      (Variables|Default|SetObjectives _returnvalue))))

(event Collision|EventActorBeginOverlap
  (params (OtherActor :type Actor%20Object%20Reference)))

(event EventTick
  (params (DeltaSeconds :type Float%20%28single-precision%29))
  (for _array_element (Variables|Default|GetAllSquads)
    (CallFunction|FindMovement _array_element)
    (Utilities|FlowControl|Delay 1.0)))

(fn ConstructionScript)

(fn SpawnSquads
  (for _array_element (Variables|Default|GetSquadsToSpawn)
    (bind _returnvalue (Utilities|GetDataTableRow "/Game/Blueprints/Units/DT_Squads.DT_Squads" _array_element)
      (:then
        (LocalVariables|SetLocal_Squad 0)
        (for (_array_element_2 _array_index) (.SquadMembers (Utilities|Struct|BreakF_Squads _returnvalue))
          (bind _returnvalue_2 (Game|SpawnActorfromClass (.UnitClass (Utilities|Struct|BreakF_Units _array_element_2)) (Transformation|GetActorTransform) "Undefined" "MultiplyWithRoot" 0 0 0))
          (if (== _array_index 0)
            (bind _output_get (LocalVariables|SetLocal_Squad (Variables|/Game/Blueprints/Units/UnitBlueprints/BP_UnitBase.BP_UnitBase_C|GetSquad _returnvalue_2)))
            (Default|SetLeader _output_get)
            (else
              (Default|AddtoSquad (LocalVariables|GetLocal_Squad) _returnvalue_2))))
        (Utilities|Array|AddUnique (Variables|Default|GetAllSquads) (LocalVariables|GetLocal_Squad))))))

(fn FindMovement
  (params (Squad :type BP%20Squad%20Object%20Reference))
  (bind _squadleader (Variables|/Game/Blueprints/Units/BP_Squad.BP_Squad_C|GetSquadLeader Squad))
  (Utilities|IsValid Squad
    (:Is%20Valid
      (bind _teamid (Default|GetTeam _squadleader))
      (Utilities|FlowControl|Sequence
        (:then_0
          (switch Utilities|FlowControl|Switch|SwitchonE_MissionType (Variables|/Game/Levels/BP_ObjectiveTracker.BP_ObjectiveTracker_C|GetObjectiveType (Variables|Default|GetObjectives))
            (:NewEnumerator1
              (bind _outactors (Actor|GetAllActorsOfClass "/Game/Blueprints/Units/BP_Squad.BP_Squad_C"))
              (for _array_element _outactors
                _))))
        (:then_1
          (for _array_element_2 (Class|AIPerceptionComponent|GetCurrentlyPerceivedActors (Class|AIController|GetAIPerceptionComponent (AI|GetAIController _squadleader)) "/Script/AIModule.AISense_Hearing")
            (bind _teamid_2 (Class|IBPRTS|GetTeam(Message) _array_element_2))
            (if (and (!= _teamid_2 0) (!= _teamid_2 _teamid))
              (AI|Components|Blackboard|SetValueasVector (AI|GetBlackboard _squadleader) (LocalVariables|GetLocalMoveToLocation) (Transformation|GetActorLocation _array_element_2)))))))))