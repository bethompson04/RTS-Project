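; RTS unit AI controller that runs the human infantry behavior tree on possession.
; AI Perception filters for "Unit"-tagged actors on another team, writing the enemy and line-of-sight flag to the blackboard.
; Losing sight starts a timer that clears both keys, so targets linger briefly, and re-sensing cancels it.
; A weapon-equipped event copies the weapon's fire rate into the blackboard.
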(event OnTargetPerceptionUpdated(AIPerception)
  (params (Actor :type Actor%20Object%20Reference) (Stimulus :type AI%20Stimulus%20Structure))
  (bind _blackboard (Variables|Default|GetBlackboard))
  (bind _teamid (Class|IBPRTS|GetTeam(Message) Actor))
  (bind _teamid_2 (Class|IBPRTS|GetTeam(Message) (Pawn|GetControlledPawn)))
  (if (and (!= _teamid_2 _teamid) (Actor|ActorHasTag Actor "Unit"))
    (if (.bSuccessfullySensed (Utilities|Struct|BreakAIStimulus Stimulus))
      (Utilities|Time|ClearandInvalidateTimerbyHandle (Variables|Default|GetEnemyTimer))
      (AI|Components|Blackboard|SetValueasBool _blackboard (Variables|Default|GetHasLineOfSight) true)
      (AI|Components|Blackboard|SetValueasObject _blackboard (Variables|Default|GetEnemyActor) Actor)
      (else
        (bind _returnvalue (Utilities|Time|SetTimerbyEvent (delegate Custom|StartEnemyTimer) (Variables|Default|GetLineOfSightTimer)))
        (Variables|Default|SetEnemyTimer _returnvalue)))))

(event Custom|StartEnemyTimer
  (bind _blackboard (Variables|Default|GetBlackboard))
  (AI|Components|Blackboard|ClearValue _blackboard (Variables|Default|GetHasLineOfSight))
  (AI|Components|Blackboard|ClearValue _blackboard (Variables|Default|GetEnemyActor)))

(event Custom|WeaponEquipped
  (params (WeaponFireRate :type Float%20%28double-precision%29))
  (AI|Components|Blackboard|SetValueasFloat (Variables|Default|GetBlackboard) (Variables|Default|GetFireRate) WeaponFireRate))

(event EventPossess
  (params (PossessedPawn :type Pawn%20Object%20Reference))
  (AI|RunBehaviorTree "/Game/Blueprints/Units/AI/BT_HumanInfantry.BT_HumanInfantry"))

(fn ConstructionScript)