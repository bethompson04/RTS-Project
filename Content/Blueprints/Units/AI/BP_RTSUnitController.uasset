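; BP_RTSUnitController is the AI controller for RTS units, running the BT_HumanInfantry behavior tree on possess.
; AI perception writes sensed other-team units to the blackboard as EnemyActor with line of sight, and a timer clears both after sight is lost.
; Perception updates from any unit also switch the pawn's stance from one specific state to another.
; Equipping a weapon passes its fire rate to the blackboard.
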(event OnTargetPerceptionUpdated(AIPerception)
  (params (Actor :type Actor%20Object%20Reference) (Stimulus :type AI%20Stimulus%20Structure))
  (bind _returnvalue (Pawn|GetControlledPawn))
  (bind _blackboard (Variables|Default|GetBlackboard))
  (bind _asbp_unit_base (Utilities|Casting|CastToBP_UnitBase _returnvalue))
  (Utilities|FlowControl|Sequence
    (:then_0
      (bind _teamid (Class|IBPRTS|GetTeam(Message) Actor))
      (bind _teamid_2 (Class|IBPRTS|GetTeam(Message) (Pawn|GetControlledPawn)))
      (if (and (!= _teamid_2 _teamid) (Actor|ActorHasTag Actor "Unit"))
        (if (.bSuccessfullySensed (Utilities|Struct|BreakAIStimulus Stimulus))
          (Utilities|Time|ClearandInvalidateTimerbyHandle (Variables|Default|GetEnemyTimer))
          (AI|Components|Blackboard|SetValueasBool _blackboard (Variables|Default|GetHasLineOfSight) true)
          (AI|Components|Blackboard|SetValueasObject _blackboard (Variables|Default|GetEnemyActor) Actor)
          (else
            (bind _returnvalue_2 (Utilities|Time|SetTimerbyEvent (delegate Custom|StartEnemyTimer) (Variables|Default|GetLineOfSightTimer)))
            (Variables|Default|SetEnemyTimer _returnvalue_2)))))
    (:then_1
      (if (and (Utilities|Enum|Equal(Enum) (Variables|/Game/Blueprints/Units/UnitBlueprints/BP_UnitBase.BP_UnitBase_C|GetStance _asbp_unit_base) "NewEnumerator2") (Actor|ActorHasTag Actor "Unit"))
        (Variables|/Game/Blueprints/Units/UnitBlueprints/BP_UnitBase.BP_UnitBase_C|SetStance _asbp_unit_base "NewEnumerator3")))))

(event Custom|StartEnemyTimer
  (bind _blackboard (Variables|Default|GetBlackboard))
  (AI|Components|Blackboard|ClearValue _blackboard (Variables|Default|GetHasLineOfSight))
  (AI|Components|Blackboard|ClearValue _blackboard (Variables|Default|GetEnemyActor)))

(event Custom|WeaponEquipped
  (params (WeaponFireRate :type Float%20%28double-precision%29))
  (AI|Components|Blackboard|SetValueasFloat (Variables|Default|GetBlackboard) (Variables|Default|GetFireRate) WeaponFireRate))

(event EventPossess
  (params (PossessedPawn :type Pawn%20Object%20Reference))
  (AI|RunBehaviorTree "/Game/Blueprints/Units/AI/BT_HumanInfantry.BT_HumanInfantry"))

(fn ConstructionScript)