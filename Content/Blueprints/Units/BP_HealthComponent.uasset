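; Health component for units that tracks current health, applies damage and signals death.
; On BeginPlay, unless hidden, it adds a screen-space widget component above the owner with a green progress bar.
; TakeDamage reports an AI damage-sense event, subtracts health and fires OnDamageTaken, plus OnDeath with the causer at zero or below.
; ManualUpdate sets the bar's fill directly and also fires OnDamageTaken, while TakeDamage itself never writes to the bar.
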(event EventBeginPlay
  (if (not (Variables|Default|GetHideHealthbar))
    (bind _returnvalue (Game|AddComponentbyClass (Components|GetOwner) "/Script/UMG.WidgetComponent" false (Math|Transform|MakeTransform "0.000000,0.000000,150.000000" "0, 0, 0" "1.000000,1.000000,1.000000")))
    (Class|WidgetComponent|SetDrawSize _returnvalue "(X=150.000000,Y=10.000000)")
    (Class|WidgetComponent|SetWidgetSpace _returnvalue "Screen")
    (Collision|SetCollisionEnabled _returnvalue "NoCollision")
    (bind _returnvalue_2 (UserInterface|CreateWidget "/Game/Blueprints/UserInterface/WBP_ProgressBar.WBP_ProgressBar_C" 0 "(R=0.000000,G=1.000000,B=0.041595,A=1.000000)" 0.0 (Components|GetOwner)))
    (bind _output_get (Variables|Default|SetProgressBar _returnvalue_2))
    (CallFunction|ManualUpdate (Variables|Default|GetCurrentHealth) (Variables|Default|GetMaxHealth))
    (UserInterface|SetWidget _returnvalue _output_get)))

(event EventTick
  (params (DeltaSeconds :type Float%20%28single-precision%29)))

(fn TakeDamage
  (params (DamageTaken :type Float%20%28double-precision%29) (DamageCauser :type BP%20Unit%20Base%20Object%20Reference))
  (Class|AISenseDamage|ReportDamageEvent (Components|GetOwner) DamageCauser DamageTaken (Transformation|GetActorLocation DamageCauser) "0, 0, 0" "Damage")
  (Variables|Default|SetCurrentHealth (- (Variables|Default|GetCurrentHealth) DamageTaken))
  (Default|CallOnDamageTaken)
  (if (<= (Variables|Default|GetCurrentHealth) 0.0)
    (Default|CallOnDeath DamageCauser)))

(fn ManualUpdate
  (params (CurrentHealth2 :type Float%20%28double-precision%29) (MaxHealth2 :type Float%20%28double-precision%29))
  (Variables|/Game/Blueprints/UserInterface/WBP_ProgressBar.WBP_ProgressBar_C|SetProgress (Variables|Default|GetProgressBar) (/ CurrentHealth2 MaxHealth2))
  (Default|CallOnDamageTaken))