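; Base RTS unit character that handles selection, squad membership, movement orders, cover, weapons, armor and inventory interaction.
; Each unit spawns its own squad at BeginPlay, follows a destination queue checked on Tick, and snaps to cover on overlap.
; Stance changes write an action state to the AI blackboard, while hustling raises speed, drains stamina and makes noise.
; On death it notifies squad and player, then spawns a corpse copying its armor and inventory.
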(event OnDeath(BP_HealthComponent)
  (params (Killer :type BP%20Unit%20Base%20Object%20Reference))
  (bind _returnvalue (AI|GetAIController Killer))
  (bind _newparam (CallFunction|GetRTSPlayer))
  (bind _teamid (Variables|Default|GetTeamID))
  (bind _equippedweapon (Variables|Default|GetEquippedWeapon))
  (bind _returnvalue_2 (Class|AIController|GetAIPerceptionComponent _returnvalue))
  (Default|MemberDied (Variables|Default|GetSquad) self)
  (if (== _teamid 1)
    (Default|CallUnitKilled _newparam self))
  (Default|CallUnitKilled (Variables|/Game/Blueprints/BP_RTSPlayerController.BP_RTSPlayerController_C|GetObjectiveTracker _newparam) _teamid)
  (Class|AIPerceptionComponent|ForgetAll _returnvalue_2)
  (Class|AIPerceptionComponent|RequestStimuliListenerUpdate _returnvalue_2)
  (Game|SpawnActorfromClass "/Game/Blueprints/Items/BP_Corpse.BP_Corpse_C" (Transformation|GetActorTransform) "Undefined" "MultiplyWithRoot" 0 (Variables|/Script/Engine.SkeletalMeshComponent|GetSkeletalMeshAsset (Variables|Character|GetMesh)) (Variables|/Game/Blueprints/Inventory/BP_InventoryComponent.BP_InventoryComponent_C|GetContents (Variables|Default|GetBP_InventoryComponent)) (Variables|Default|GetStance) (Variables|/Script/Engine.StaticMeshComponent|GetStaticMesh (Variables|Default|GetHelmetMesh)) (Variables|/Script/Engine.StaticMeshComponent|GetStaticMesh (Variables|Default|GetChestMesh)) (Variables|/Script/Engine.StaticMeshComponent|GetStaticMesh (Variables|Default|GetLShoulderMesh)) (Variables|/Script/Engine.StaticMeshComponent|GetStaticMesh (Variables|Default|GetRShoulderMesh)) (Variables|/Script/Engine.StaticMeshComponent|GetStaticMesh (Variables|Default|GetBeltMesh)) (Variables|/Script/Engine.StaticMeshComponent|GetStaticMesh (Variables|Default|GetLThighMesh)) (Variables|/Script/Engine.StaticMeshComponent|GetStaticMesh (Variables|Default|GetRThighMesh)) (Variables|/Script/Engine.StaticMeshComponent|GetStaticMesh (Variables|Default|GetLArmMesh)) (Variables|/Script/Engine.StaticMeshComponent|GetStaticMesh (Variables|Default|GetRArmMesh)) (Variables|/Script/Engine.StaticMeshComponent|GetStaticMesh (Variables|Default|GetLLegMesh)) (Variables|/Script/Engine.StaticMeshComponent|GetStaticMesh (Variables|Default|GetRLegMesh)) 0) ; Oh my God
  (if (!= (Math|Random|RandomIntegerinRange 0 1) 0)
    _
    (else
      (Audio|PlaySoundatLocation "/Game/Assets/Sounds/144338__jpolito__scream.144338__jpolito__scream" (Transformation|GetActorLocation) "0, 0, 0" 1.0 1.0 0.0 0 0 0 0)))
  (Utilities|IsValid _equippedweapon
    (:Is%20Valid
      (Actor|DestroyActor _equippedweapon))
    (:Is%20Not%20Valid
      _))
  (Actor|DestroyActor))

(event Custom|ReloadUnitWeapon
  (CallFunction|ReloadWeapon))

(event Custom|EquipFirstWeapon
  (bind _bp_inventorycomponent (Variables|Default|GetBP_InventoryComponent))
  (bind (_itemid _index) (Default|HasWeapon _bp_inventorycomponent))
  (if (!= _index -1)
    (Default|OwnerUseItem _bp_inventorycomponent _itemid _index 1)))

(event EventBeginPlay
  (Utilities|FlowControl|Sequence
    (:then_0
      (Rendering|SetVisibility (Variables|Default|GetSelectionMesh) false false)
      (CallFunction|LoneWolf))
    (:then_1
      (CallFunction|EquipArmor))))

(event EventSetDestination
  (params (Add :type Boolean) (ToCover :type Boolean) (Destination :type Vector :default "0, 0, 0"))
  (Variables|Default|SetTakingCover ToCover)
  (CallFunction|SetUnitDestination Add ToCover Destination))

(event EventLeaveCover
  (Variables|Default|SetCover 0)
  (Variables|Default|SetTakingCover false))

(event Collision|EventActorBeginOverlap
  (params (OtherActor :type Actor%20Object%20Reference))
  (Utilities|IsValid OtherActor
    (:Is%20Valid
      (if true
        (if (and (Actor|ActorHasTag OtherActor "Cover") (Variables|Default|GetTakingCover))
          (CallFunction|TakeCover))))))

(event EventRemovedfromSquad
  (params (ToNewSquad :type Boolean))
  (if ToNewSquad
    (CallFunction|LoneWolf)))

(event EventHustleUnit
  (Variables|Default|SetIsHustling true)
  (Variables|/Script/Engine.CharacterMovementComponent|SetMaxWalkSpeed (Variables|Character|GetCharacterMovement) 6e+02)
  (CallFunction|ChangeStance "NewEnumerator8")
  (Class|Actor|MakeNoise 1.0 self (Transformation|GetActorLocation) 1e+04 "Sound"))

(event EventTick
  (params (DeltaSeconds :type Float%20%28single-precision%29))
  (bind _destinationsarray (Variables|Default|GetDestinationsArray))
  (Utilities|FlowControl|Sequence
    (:then_0
      (if (Variables|Default|GetIsHustling)
        (Variables|Default|SetStamina (- (Variables|Default|GetStamina) (* DeltaSeconds 2.0)))
        (elif (<= (Variables|Default|GetStamina) (Variables|Default|GetMaxStamina))
          (Variables|Default|SetStamina (+ (Variables|Default|GetStamina) DeltaSeconds)))))
    (:then_1
      (if (Utilities|Array|IsValidIndex _destinationsarray)
        (Variables|Default|SetCurrentDestination (Utilities|Array|Get(acopy) _destinationsarray))
        (if (< (Math|Vector|VectorLength (- (Transformation|GetActorLocation) (Variables|Default|GetCurrentDestination))) 1.2e+02)
          (CallFunction|CheckforNextDestination))))
    (:then_2)))

(event MouseInput|EventActorBeginCursorOver
  (Rendering|SetVisibility (Variables|Default|GetSelectionMesh) true false))

(event MouseInput|EventActorEndCursorOver
  (if (not (Variables|Default|GetIsSelected))
    (Rendering|SetVisibility (Variables|Default|GetSelectionMesh) false false)))

(event EventDeSelected
  (CallFunction|Deselect))

(event EventCancelHustle
  (Variables|Default|SetIsHustling false)
  (Variables|/Script/Engine.CharacterMovementComponent|SetMaxWalkSpeed (Variables|Character|GetCharacterMovement) 3e+02)
  (CallFunction|ChangeStance "NewEnumerator7"))

(event EventSelected
  (CallFunction|Select))

(event EventToCover
  (params (TargetCover :type BP%20Unit%20Cover%20Object%20Reference))
  (Variables|Default|SetCover TargetCover)
  (Variables|Default|SetTakingCover true))

(fn ConstructionScript)

(fn Select
  (bind _selectionmesh (Variables|Default|GetSelectionMesh))
  (Variables|Default|SetIsSelected true)
  (Rendering|SetVisibility _selectionmesh true false)
  (Default|ShowHealth (Variables|Default|GetBP_HealthComponent) true false)
  (if (== (Variables|/Game/Blueprints/Units/BP_Squad.BP_Squad_C|GetSquadLeader (Variables|Default|GetSquad)) self)
    (Rendering|Material|SetMaterial _selectionmesh 0 "/Game/Assets/Materials/Selection_DiscSquadLead.Selection_DiscSquadLead")
    (else
      (Rendering|Material|SetMaterial _selectionmesh 0 "/Game/Assets/Materials/Selection_Disc.Selection_Disc"))))

(fn Deselect
  (Variables|Default|SetIsSelected false)
  (Rendering|SetVisibility (Variables|Default|GetSelectionMesh) false false)
  (Default|ShowHealth (Variables|Default|GetBP_HealthComponent) false false))

(fn SetUnitDestination
  (params (Add :type Boolean) (ToCover :type Boolean) (Destination :type Vector))
  (bind _destinationsarray (Variables|Default|GetDestinationsArray))
  (if Add
    (Utilities|Array|AddUnique _destinationsarray Destination)
    (Development|PrintText "Added Destination")
    (else
      (AI|Navigation|MovetoLocation (AI|GetAIController self) Destination 16.0 true true true true "/Script/AIModule.NavFilter_AIControllerDefault")
      (Utilities|Array|Clear _destinationsarray)
      (Utilities|Array|AddUnique _destinationsarray Destination)))
  (return))

(fn CheckforNextDestination
  (bind _destinationsarray (Variables|Default|GetDestinationsArray))
  (if (Utilities|Array|IsValidIndex _destinationsarray)
    (Utilities|Array|RemoveIndex _destinationsarray)
    (if (Utilities|Array|IsValidIndex _destinationsarray)
      (CallFunction|SetUnitDestination false false (Utilities|Array|Get(acopy) _destinationsarray))
      (else
        (Variables|Default|SetIsHustling false)
        (Variables|/Script/Engine.CharacterMovementComponent|SetMaxWalkSpeed (Variables|Character|GetCharacterMovement) 3e+02)
        (CallFunction|ChangeStance "NewEnumerator2")))))

(fn TakeCover
  (bind _cover (Variables|Default|GetCover))
  (Transformation|SetWorldTransform (Variables|Collision|GetCapsuleComponent) (Transformation|GetActorTransform _cover) false false)
  (switch Utilities|FlowControl|Switch|SwitchonE_CoverType (Variables|/Game/Blueprints/Cover/BP_UnitCover.BP_UnitCover_C|GetCoverType _cover)
    (:NewEnumerator0
      (CallFunction|ChangeStance "NewEnumerator0"))
    (:NewEnumerator1
      (CallFunction|ChangeStance "NewEnumerator1"))
    (:NewEnumerator2
      (CallFunction|ChangeStance "NewEnumerator4"))))

(fn LoneWolf
  (Utilities|IsValid (Variables|Default|GetSquad)
    (:Is%20Valid
      (Default|RemovefromSquad (Variables|Default|GetSquad) self))
    (:Is%20Not%20Valid
      _))
  (bind _returnvalue (Game|SpawnActorfromClass "/Game/Blueprints/Units/BP_Squad.BP_Squad_C" (Transformation|GetActorTransform) "Undefined" "MultiplyWithRoot" 0 0))
  (bind _output_get (Variables|Default|SetSquad _returnvalue))
  (Default|AddtoSquad _output_get self))

(fn UnitInteractwith
  (bind _returnvalue (Transformation|GetActorLocation))
  (bind _bp_inventorycomponent (Variables|Default|GetBP_InventoryComponent))
  (Variables|Default|SetToInteract true)
  (bind _targetactor (Variables|/Game/Blueprints/Inventory/BP_InventoryComponent.BP_InventoryComponent_C|GetTargetActor _bp_inventorycomponent)
    (:then
      (Development|PrintText (Utilities|Text|FormatText "Interact with: {target}" _targetactor))
      (if (> (Math|Vector|Distance(Vector) (Transformation|GetActorLocation _targetactor) _returnvalue) (Variables|/Game/Blueprints/Inventory/BP_InventoryComponent.BP_InventoryComponent_C|GetPickupRange _bp_inventorycomponent))
        (CallFunction|SetUnitDestination false false (+ (Transformation|GetActorLocation _targetactor) (* (- _returnvalue (Transformation|GetActorLocation _targetactor)) 0.1)))
        (else
          (Default|Interact _bp_inventorycomponent))))
    (:else)))

(fn SetInteractTarget
  (params (InteractTarget :type Actor%20Object%20Reference))
  (bind _output_get (Variables|/Game/Blueprints/Inventory/BP_InventoryComponent.BP_InventoryComponent_C|SetTargetActor (Variables|Default|GetBP_InventoryComponent) InteractTarget))
  (Class|BPIInteractInterface|Lookat(Message) _output_get))

(fn ReloadWeapon
  (bind _bp_inventorycomponent (Variables|Default|GetBP_InventoryComponent))
  (bind _equippedweapon (Variables|Default|GetEquippedWeapon))
  (bind _magsize (Variables|/Game/Blueprints/Items/Weapons/BP_WeaponBase.BP_WeaponBase_C|GetMagSize _equippedweapon))
  (LocalVariables|SetLocal_Index 0)
  (LocalVariables|SetLocal_NeedMoreAmmo true)
  (bind (_indexes _totalcount) (Default|FindSpecificContents _bp_inventorycomponent (.RowName (Utilities|Struct|BreakDataTableRowHandle (Variables|/Game/Blueprints/Items/Weapons/BP_WeaponBase.BP_WeaponBase_C|GetAmmoStats _equippedweapon)))))
  (if (> _totalcount 0)
    (while (LocalVariables|GetLocal_NeedMoreAmmo)
      (if (>= (.Quantity (Utilities|Struct|BreakF_SlotStruct (Utilities|Array|Get(acopy) (Variables|/Game/Blueprints/Inventory/BP_InventoryComponent.BP_InventoryComponent_C|GetContents _bp_inventorycomponent) (Utilities|Array|Get(acopy) _indexes (LocalVariables|GetLocal_Index))))) _magsize)
        (Default|RemovefromInventory _bp_inventorycomponent (Utilities|Array|Get(acopy) _indexes (LocalVariables|GetLocal_Index)) true _magsize)
        (LocalVariables|SetLocal_ReloadAmount _magsize)
        (LocalVariables|SetLocal_NeedMoreAmmo false)
        (else
          (LocalVariables|SetLocal_ReloadAmount (.Quantity (Utilities|Struct|BreakF_SlotStruct (Utilities|Array|Get(acopy) (Variables|/Game/Blueprints/Inventory/BP_InventoryComponent.BP_InventoryComponent_C|GetContents _bp_inventorycomponent) (Utilities|Array|Get(acopy) _indexes (LocalVariables|GetLocal_Index))))))
          (Default|RemovefromInventory (Variables|Default|GetBP_InventoryComponent) (Utilities|Array|Get(acopy) _indexes (LocalVariables|GetLocal_Index)) true (.Quantity (Utilities|Struct|BreakF_SlotStruct (Utilities|Array|Get(acopy) (Variables|/Game/Blueprints/Inventory/BP_InventoryComponent.BP_InventoryComponent_C|GetContents _bp_inventorycomponent) (Utilities|Array|Get(acopy) _indexes (LocalVariables|GetLocal_Index))))))
          (bind _result (Math|Integer|IncrementInt (LocalVariables|GetLocal_Index))
            (:%20%20
              (bind _output_get (LocalVariables|SetLocal_Index _result))
              (if (>= _output_get (Utilities|Array|Length _indexes))
                (LocalVariables|SetLocal_NeedMoreAmmo false)))))))
    (Default|Reload _equippedweapon (LocalVariables|GetLocal_ReloadAmount))))

(fn Interacting
  (params (UseTime :type Float%20%28double-precision%29))
  (if (> UseTime 0.0)
    (CallFunction|ChangeStance "NewEnumerator6")
    (AI|Components|Blackboard|SetValueasFloat (Variables|/Script/AIModule.AIController|GetBlackboard (AI|GetAIController self)) (LocalVariables|GetLocal_InteractTime) UseTime))
  (return true))

(fn EquipItem
  (params (ItemToEquip :type BP%20Weapon%20Base%20Object%20Reference))
  (bind _output_get (Variables|Default|SetEquippedWeapon ItemToEquip))
  (Default|SetWeaponOwner _output_get self)
  (Transformation|AttachComponentToComponent _output_get (Variables|Character|GetMesh) (Variables|Default|GetWeaponSocketName) "SnapToTarget" "SnapToTarget" "SnapToTarget" true)
  (Variables|/Game/Blueprints/Items/Weapons/BP_WeaponBase.BP_WeaponBase_C|SetEquipped (Variables|Default|GetEquippedWeapon) true)
  (bind _asbp_rtsunit_controller (Utilities|Casting|CastToBP_RTSUnitController (AI|GetAIController self)))
  (Default|WeaponEquipped _asbp_rtsunit_controller (Variables|/Game/Blueprints/Items/Weapons/BP_WeaponBase.BP_WeaponBase_C|GetWeaponFireRate (Variables|Default|GetEquippedWeapon))))

(fn AttackOrder
  (params (ActorToTarget :type Actor%20Object%20Reference) (TargetLocation :type Vector))
  (bind _equippedweapon (Variables|Default|GetEquippedWeapon))
  (Utilities|IsValid (Variables|Default|GetEquippedWeapon)
    (:Is%20Valid
      (Utilities|IsValid ActorToTarget
        (:Is%20Valid
          (bind _output_get (Variables|Default|SetAttackTarget ActorToTarget))
          (AI|Components|Blackboard|SetValueasObject (AI|GetBlackboard 0) (LocalVariables|GetLocal_EnemyActor) _output_get)
          (Default|UseWeapon _equippedweapon (Transformation|GetActorLocation _output_get)))
        (:Is%20Not%20Valid
          (Default|UseWeapon _equippedweapon TargetLocation))))))

(fn ChangeStance
  (params (NewStance :type E_UnitPosition%20Enum :default "NewEnumerator2"))
  (bind _self self)
  (bind _local_actionstate (LocalVariables|GetLocal_ActionState))
  (bind _returnvalue (AI|GetAIController _self))
  (bind _blackboard (Variables|/Script/AIModule.AIController|GetBlackboard _returnvalue))
  (bind _output_get (Variables|Default|SetStance NewStance))
  (switch Utilities|FlowControl|Switch|SwitchonE_UnitPosition _output_get
    (:NewEnumerator2
      (AI|Components|Blackboard|SetValueasEnum _blackboard _local_actionstate :!label _label))
    (:NewEnumerator4
      (goto _label))
    (:NewEnumerator3
      (goto _label))
    (:NewEnumerator0
      (AI|Components|Blackboard|SetValueasEnum _blackboard _local_actionstate 3 :!label _label_2))
    (:NewEnumerator1
      (goto _label_2))
    (:NewEnumerator7
      (AI|Components|Blackboard|SetValueasEnum _blackboard _local_actionstate 1))
    (:NewEnumerator8
      (AI|Components|Blackboard|SetValueasEnum _blackboard _local_actionstate 2))
    (:NewEnumerator6
      (AI|Components|Blackboard|SetValueasEnum _blackboard _local_actionstate 4))))

(fn EquipArmor
  (bind _beltmesh (Variables|Default|GetBeltMesh))
  (bind _mesh (Variables|Character|GetMesh))
  (bind _larmmesh (Variables|Default|GetLArmMesh))
  (bind _rarmmesh (Variables|Default|GetRArmMesh))
  (bind _mesh_2 (Variables|Character|GetMesh))
  (bind _helmetmesh (Variables|Default|GetHelmetMesh))
  (bind _chestmesh (Variables|Default|GetChestMesh))
  (bind _lshouldermesh (Variables|Default|GetLShoulderMesh))
  (bind _rshouldermesh (Variables|Default|GetRShoulderMesh))
  (bind _lthighmesh (Variables|Default|GetLThighMesh))
  (bind _llegmesh (Variables|Default|GetLLegMesh))
  (bind _rthighmesh (Variables|Default|GetRThighMesh))
  (bind _rlegmesh (Variables|Default|GetRLegMesh))
  (bind _mesh_3 (Variables|Character|GetMesh))
  (Utilities|FlowControl|Sequence
    (:then_0
      (Transformation|SetWorldTransform _helmetmesh (Transformation|GetSocketTransform (Variables|Character|GetMesh) "HelmetSocket" "RTS_World") false true)
      (Transformation|AttachComponentToComponent _helmetmesh _mesh_2 "HelmetSocket" "KeepWorld" "KeepWorld" "KeepWorld" true)
      (Transformation|SetWorldTransform _chestmesh (Transformation|GetSocketTransform (Variables|Character|GetMesh) "ChestSocket" "RTS_World") false true)
      (Transformation|AttachComponentToComponent _chestmesh _mesh_2 "ChestSocket" "KeepWorld" "KeepWorld" "KeepWorld" true)
      (Transformation|SetWorldTransform _lshouldermesh (Transformation|GetSocketTransform (Variables|Character|GetMesh) "LShoulderSocket" "RTS_World") false true)
      (Transformation|AttachComponentToComponent _lshouldermesh _mesh_2 "LShoulderSocket" "KeepWorld" "KeepWorld" "KeepWorld" true)
      (Transformation|SetWorldTransform _rshouldermesh (Transformation|GetSocketTransform (Variables|Character|GetMesh) "RShoulderSocket" "RTS_World") false true)
      (Transformation|AttachComponentToComponent _rshouldermesh _mesh_2 "RShoulderSocket" "KeepWorld" "KeepWorld" "KeepWorld" true))
    (:then_1
      (Transformation|SetWorldTransform _beltmesh (Transformation|GetSocketTransform (Variables|Character|GetMesh) "HipsSocket" "RTS_World") false true)
      (Transformation|AttachComponentToComponent _beltmesh _mesh_3 "HipsSocket" "KeepWorld" "KeepWorld" "KeepWorld" true)
      (Transformation|SetWorldTransform _larmmesh (Transformation|GetSocketTransform (Variables|Character|GetMesh) "LArmSocket" "RTS_World") false true)
      (Transformation|AttachComponentToComponent _larmmesh _mesh_3 "LArmSocket" "KeepWorld" "KeepWorld" "KeepWorld" true)
      (Transformation|SetWorldTransform _rarmmesh (Transformation|GetSocketTransform (Variables|Character|GetMesh) "RArmSocket" "RTS_World") false true)
      (Transformation|AttachComponentToComponent _rarmmesh _mesh_3 "RArmSocket" "KeepWorld" "KeepWorld" "KeepWorld" true))
    (:then_2
      (Transformation|SetWorldTransform _lthighmesh (Transformation|GetSocketTransform (Variables|Character|GetMesh) "LThighSocket" "RTS_World") false true)
      (Transformation|AttachComponentToComponent _lthighmesh _mesh "LThighSocket" "KeepWorld" "KeepWorld" "KeepWorld" true)
      (Transformation|SetWorldTransform _llegmesh (Transformation|GetSocketTransform (Variables|Character|GetMesh) "LLegSocket" "RTS_World") false true)
      (Transformation|AttachComponentToComponent _llegmesh _mesh "LLegSocket" "KeepWorld" "KeepWorld" "KeepWorld" true)
      (Transformation|SetWorldTransform _rthighmesh (Transformation|GetSocketTransform (Variables|Character|GetMesh) "RThighSocket" "RTS_World") false true)
      (Transformation|AttachComponentToComponent _rthighmesh _mesh "RThighSocket" "KeepWorld" "KeepWorld" "KeepWorld" true)
      (Transformation|SetWorldTransform _rlegmesh (Transformation|GetSocketTransform (Variables|Character|GetMesh) "RLegSocket" "RTS_World") false true)
      (Transformation|AttachComponentToComponent _rlegmesh _mesh "RLegSocket" "KeepWorld" "KeepWorld" "KeepWorld" true))))

(fn GetTeam
  (return (Variables|Default|GetTeamID)))