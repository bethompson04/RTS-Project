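; Base class for a selectable RTS squad unit that moves, takes cover, fights and interacts through inventory and health components.
; It spawns its own one-member squad at start and notifies the squad on death.
; Move orders go to the AI controller with a waypoint array advanced on Tick, alongside hustle stamina and stance-based debug-style materials.
; Cover overlaps snap the unit into a stance; equipped weapons handle attacks and reload from inventory ammo.
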(event OnDeath(BP_HealthComponent)
  (params (Killer :type BP%20Unit%20Base%20Object%20Reference))
  (bind _returnvalue (AI|GetAIController Killer))
  (bind _returnvalue_2 (Class|AIController|GetAIPerceptionComponent _returnvalue))
  (Default|MemberDied (Variables|Default|GetSquad) self)
  (Actor|DestroyActor)
  (Class|AIPerceptionComponent|ForgetAll _returnvalue_2)
  (Class|AIPerceptionComponent|RequestStimuliListenerUpdate _returnvalue_2))

(event Custom|ReloadUnitWeapon
  (CallFunction|ReloadWeapon))

(event EventBeginPlay
  (bind _bp_inventorycomponent (Variables|Default|GetBP_InventoryComponent))
  (Rendering|SetVisibility (Variables|Default|GetSelectionMesh) false false)
  (CallFunction|LoneWolf)
  (bind (_itemid _index) (Default|HasWeapon _bp_inventorycomponent))
  (if (!= _index -1)
    (Default|OwnerUseItem _bp_inventorycomponent _itemid _index 1)))

(event EventSetDestination
  (params (Add :type Boolean) (ToCover :type Boolean) (Destination :type Vector :default "0, 0, 0"))
  (Variables|Default|SetTakingCover ToCover)
  (CallFunction|SetUnitDestination Add ToCover Destination)
  (Class|AISenseHearing|ReportNoiseEvent (Transformation|GetActorLocation) 1.0 self 3e+03 "Unit"))

(event EventLeaveCover
  (Variables|Default|SetCover 0)
  (Variables|Default|SetTakingCover false))

(event Collision|EventActorBeginOverlap
  (params (OtherActor :type Actor%20Object%20Reference))
  (Utilities|IsValid OtherActor
    (:Is%20Valid
      (if true
        (if (and (Actor|ActorHasTag OtherActor "Cover") (Variables|Default|GetTakingCover))
          (CallFunction|TakeCover))))))

(event EventRemovedfromSquad
  (params (ToNewSquad :type Boolean))
  (if ToNewSquad
    (CallFunction|LoneWolf)))

(event EventHustleUnit
  (Variables|Default|SetIsHustling true)
  (Variables|/Script/Engine.CharacterMovementComponent|SetMaxWalkSpeed (Variables|Character|GetCharacterMovement) 6e+02)
  (Variables|Default|SetStance "NewEnumerator8"))

(event EventTick
  (params (DeltaSeconds :type Float%20%28single-precision%29))
  (bind _mesh (Variables|Character|GetMesh))
  (bind _destinationsarray (Variables|Default|GetDestinationsArray))
  (Utilities|FlowControl|Sequence
    (:then_0
      (if (Variables|Default|GetIsHustling)
        (Variables|Default|SetStamina (- (Variables|Default|GetStamina) (* DeltaSeconds 2.0)))
        (elif (<= (Variables|Default|GetStamina) (Variables|Default|GetMaxStamina))
          (Variables|Default|SetStamina (+ (Variables|Default|GetStamina) DeltaSeconds)))))
    (:then_1
      (if (Utilities|Array|IsValidIndex _destinationsarray)
        (Variables|Default|SetCurrentDestination (Utilities|Array|Get(acopy) _destinationsarray))
        (if (< (Math|Vector|VectorLength (- (Transformation|GetActorLocation) (Variables|Default|GetCurrentDestination))) 1.2e+02)
          (CallFunction|CheckforNextDestination))))
    (:then_2)
    (:then_3
      (switch Utilities|FlowControl|Switch|SwitchonE_UnitPosition (Variables|Default|GetStance)
        (:NewEnumerator2
          (Rendering|Material|SetMaterial _mesh 0 "/AnimationSharing/AnimSharingBase.AnimSharingBase"))
        (:NewEnumerator4
          (Rendering|Material|SetMaterial _mesh 0 "/AnimationSharing/AnimSharingRed.AnimSharingRed"))
        (:NewEnumerator3
          (Rendering|Material|SetMaterial _mesh 0 "/AnimationSharing/AnimSharingGreen.AnimSharingGreen"))
        (:NewEnumerator0
          (Rendering|Material|SetMaterial _mesh 0 "/Engine/Tutorial/SubEditors/TutorialAssets/Character/TutorialTPP_Mat.TutorialTPP_Mat" :!label _label))
        (:NewEnumerator1
          (goto _label))))))

(event MouseInput|EventActorBeginCursorOver
  (Rendering|SetVisibility (Variables|Default|GetSelectionMesh) true false))

(event MouseInput|EventActorEndCursorOver
  (if (not (Variables|Default|GetIsSelected))
    (Rendering|SetVisibility (Variables|Default|GetSelectionMesh) false false)))

(event EventDeSelected
  (CallFunction|Deselect))

(event EventCancelHustle
  (Variables|Default|SetIsHustling false)
  (Variables|/Script/Engine.CharacterMovementComponent|SetMaxWalkSpeed (Variables|Character|GetCharacterMovement) 3e+02)
  (Variables|Default|SetStance "NewEnumerator7"))

(event EventSelected
  (CallFunction|Select))

(event EventToCover
  (params (TargetCover :type BP%20Unit%20Cover%20Object%20Reference))
  (Variables|Default|SetCover TargetCover)
  (Variables|Default|SetTakingCover true))

(fn ConstructionScript)

(fn Select
  (bind _selectionmesh (Variables|Default|GetSelectionMesh))
  (Variables|Default|SetIsSelected true)
  (Rendering|SetVisibility _selectionmesh true false)
  (if (== (Variables|/Game/Blueprints/Units/BP_Squad.BP_Squad_C|GetSquadLeader (Variables|Default|GetSquad)) self)
    (Rendering|Material|SetMaterial _selectionmesh 0 "/AnimationSharing/AnimSharingBlue.AnimSharingBlue")
    (else
      (Rendering|Material|SetMaterial _selectionmesh 0 "/AnimationSharing/AnimSharingBase.AnimSharingBase"))))

(fn Deselect
  (Variables|Default|SetIsSelected false)
  (Rendering|SetVisibility (Variables|Default|GetSelectionMesh) false false))

(fn SetUnitDestination
  (params (Add :type Boolean) (ToCover :type Boolean) (Destination :type Vector))
  (bind _destinationsarray (Variables|Default|GetDestinationsArray))
  (if Add
    (Utilities|Array|AddUnique _destinationsarray Destination)
    (Development|PrintText "Added Destination")
    (else
      (AI|Navigation|MovetoLocation (AI|GetAIController self) Destination 16.0 true true true true "/Script/AIModule.NavFilter_AIControllerDefault")
      (Utilities|Array|Clear _destinationsarray)
      (Utilities|Array|AddUnique _destinationsarray Destination)
      (Development|PrintText "Set Destination")))
  (return))

(fn CheckforNextDestination
  (bind _destinationsarray (Variables|Default|GetDestinationsArray))
  (if (Utilities|Array|IsValidIndex _destinationsarray)
    (Utilities|Array|RemoveIndex _destinationsarray)
    (if (Utilities|Array|IsValidIndex _destinationsarray)
      (CallFunction|SetUnitDestination false false (Utilities|Array|Get(acopy) _destinationsarray))
      (else
        (Variables|Default|SetIsHustling false)
        (Variables|/Script/Engine.CharacterMovementComponent|SetMaxWalkSpeed (Variables|Character|GetCharacterMovement) 3e+02)))))

(fn TakeCover
  (bind _cover (Variables|Default|GetCover))
  (Transformation|SetWorldTransform (Variables|Collision|GetCapsuleComponent) (Transformation|GetActorTransform _cover) false false)
  (switch Utilities|FlowControl|Switch|SwitchonE_CoverType (Variables|/Game/Blueprints/Cover/BP_UnitCover.BP_UnitCover_C|GetCoverType _cover)
    (:NewEnumerator0
      (Variables|Default|SetStance "NewEnumerator0"))
    (:NewEnumerator1
      (Variables|Default|SetStance "NewEnumerator1"))
    (:NewEnumerator2
      (Variables|Default|SetStance "NewEnumerator4")))
  (Development|PrintString "In Cover!"))

(fn LoneWolf
  (Utilities|IsValid (Variables|Default|GetSquad)
    (:Is%20Valid
      (Default|RemovefromSquad (Variables|Default|GetSquad) self))
    (:Is%20Not%20Valid
      _))
  (bind _returnvalue (Game|SpawnActorfromClass "/Game/Blueprints/Units/BP_Squad.BP_Squad_C" (Transformation|GetActorTransform) "Undefined" "MultiplyWithRoot" 0 0))
  (bind _output_get (Variables|Default|SetSquad _returnvalue))
  (Default|AddtoSquad _output_get self))

(fn UnitInteractwith
  (bind _returnvalue (Transformation|GetActorLocation))
  (bind _bp_inventorycomponent (Variables|Default|GetBP_InventoryComponent))
  (Variables|Default|SetToInteract true)
  (bind _targetactor (Variables|/Game/Blueprints/Inventory/BP_InventoryComponent.BP_InventoryComponent_C|GetTargetActor _bp_inventorycomponent)
    (:then
      (Development|PrintText (Utilities|Text|FormatText "Interact with: {target}" _targetactor))
      (if (> (Math|Vector|Distance(Vector) (Transformation|GetActorLocation _targetactor) _returnvalue) (Variables|/Game/Blueprints/Inventory/BP_InventoryComponent.BP_InventoryComponent_C|GetPickupRange _bp_inventorycomponent))
        (CallFunction|SetUnitDestination false false (+ (Transformation|GetActorLocation _targetactor) (* (- _returnvalue (Transformation|GetActorLocation _targetactor)) 0.1)))
        (else
          (Default|Interact _bp_inventorycomponent))))
    (:else)))

(fn SetInteractTarget
  (params (InteractTarget :type Actor%20Object%20Reference))
  (bind _output_get (Variables|/Game/Blueprints/Inventory/BP_InventoryComponent.BP_InventoryComponent_C|SetTargetActor (Variables|Default|GetBP_InventoryComponent) InteractTarget))
  (Class|BPIInteractInterface|Lookat(Message) _output_get))

(fn ReloadWeapon
  (bind _bp_inventorycomponent (Variables|Default|GetBP_InventoryComponent))
  (bind _equippedweapon (Variables|Default|GetEquippedWeapon))
  (bind _magsize (Variables|/Game/Blueprints/Items/Weapons/BP_WeaponBase.BP_WeaponBase_C|GetMagSize _equippedweapon))
  (LocalVariables|SetLocal_Index 0)
  (LocalVariables|SetLocal_NeedMoreAmmo true)
  (bind (_indexes _totalcount) (Default|FindSpecificContents _bp_inventorycomponent (.RowName (Utilities|Struct|BreakDataTableRowHandle (Variables|/Game/Blueprints/Items/Weapons/BP_WeaponBase.BP_WeaponBase_C|GetAmmoStats _equippedweapon)))))
  (if (> _totalcount 0)
    (while (LocalVariables|GetLocal_NeedMoreAmmo)
      (if (>= (.Quantity (Utilities|Struct|BreakF_SlotStruct (Utilities|Array|Get(acopy) (Variables|/Game/Blueprints/Inventory/BP_InventoryComponent.BP_InventoryComponent_C|GetContents _bp_inventorycomponent) (Utilities|Array|Get(acopy) _indexes (LocalVariables|GetLocal_Index))))) _magsize)
        (Default|RemovefromInventory _bp_inventorycomponent (Utilities|Array|Get(acopy) _indexes (LocalVariables|GetLocal_Index)) true _magsize)
        (LocalVariables|SetLocal_ReloadAmount _magsize)
        (LocalVariables|SetLocal_NeedMoreAmmo false)
        (else
          (LocalVariables|SetLocal_ReloadAmount (.Quantity (Utilities|Struct|BreakF_SlotStruct (Utilities|Array|Get(acopy) (Variables|/Game/Blueprints/Inventory/BP_InventoryComponent.BP_InventoryComponent_C|GetContents _bp_inventorycomponent) (Utilities|Array|Get(acopy) _indexes (LocalVariables|GetLocal_Index))))))
          (Default|RemovefromInventory (Variables|Default|GetBP_InventoryComponent) (Utilities|Array|Get(acopy) _indexes (LocalVariables|GetLocal_Index)) true (.Quantity (Utilities|Struct|BreakF_SlotStruct (Utilities|Array|Get(acopy) (Variables|/Game/Blueprints/Inventory/BP_InventoryComponent.BP_InventoryComponent_C|GetContents _bp_inventorycomponent) (Utilities|Array|Get(acopy) _indexes (LocalVariables|GetLocal_Index))))))
          (bind _result (Math|Integer|IncrementInt (LocalVariables|GetLocal_Index))
            (:%20%20
              (bind _output_get (LocalVariables|SetLocal_Index _result))
              (if (>= _output_get (Utilities|Array|Length _indexes))
                (LocalVariables|SetLocal_NeedMoreAmmo false)))))))
    (Default|Reload _equippedweapon (LocalVariables|GetLocal_ReloadAmount))))

(fn Interacting
  (params (UseTime :type Float%20%28double-precision%29))
  (if (> UseTime 0.0)
    (Class|SubmixEffectDelayStatics|SetDelayLength (Utilities|Struct|MakeSubmixEffectDelaySettings 2e+03 4e+02 1e+03) UseTime))
  (return true))

(fn EquipItem
  (params (ItemToEquip :type BP%20Weapon%20Base%20Object%20Reference))
  (bind _output_get (Variables|Default|SetEquippedWeapon ItemToEquip))
  (Default|SetWeaponOwner _output_get self)
  (Transformation|AttachComponentToComponent _output_get (Variables|Character|GetMesh) (Variables|Default|GetWeaponSocketName) "SnapToTarget" "SnapToTarget" "SnapToTarget" true)
  (bind _asbp_rtsunit_controller (Utilities|Casting|CastToBP_RTSUnitController (AI|GetAIController self)))
  (Default|WeaponEquipped _asbp_rtsunit_controller (Variables|/Game/Blueprints/Items/Weapons/BP_WeaponBase.BP_WeaponBase_C|GetWeaponFireRate (Variables|Default|GetEquippedWeapon))))

(fn AttackOrder
  (params (ActorToTarget :type Actor%20Object%20Reference) (TargetLocation :type Vector))
  (bind _equippedweapon (Variables|Default|GetEquippedWeapon))
  (Utilities|IsValid (Variables|Default|GetEquippedWeapon)
    (:Is%20Valid
      (Utilities|IsValid ActorToTarget
        (:Is%20Valid
          (bind _output_get (Variables|Default|SetAttackTarget ActorToTarget))
          (Default|UseWeapon _equippedweapon (Transformation|GetActorLocation _output_get)))
        (:Is%20Not%20Valid
          (Default|UseWeapon _equippedweapon TargetLocation))))))

(fn GetTeam
  (return (Variables|Default|GetTeamID)))