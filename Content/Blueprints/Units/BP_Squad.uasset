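; Squad actor that groups units and relays selection, hustle, cover and attack orders to them, cycles their stance, and destroys itself when emptied.
; The first member serves as leader and receives move orders, with followers given destinations after a short delay.
; A pair moves side by side, while larger squads keep their offsets from the leader, randomly pulling far stragglers inward.
; Cover orders assign members by index to the cover's points.
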(event EventBeginPlay
  (CallFunction|SetLeader))

(event Collision|EventActorBeginOverlap
  (params (OtherActor :type Actor%20Object%20Reference)))

(event EventTick
  (params (DeltaSeconds :type Float%20%28single-precision%29)))

(event EventSelected
  (for _array_element (Variables|Default|GetSquadMembers)
    (Class|IBPRTS|Selected(Message) _array_element)))

(event EventDeselected
  (for _array_element (Variables|Default|GetSquadMembers)
    (Class|IBPRTS|Deselected(Message) _array_element)))

(event EventHustleUnit
  (for _array_element (Variables|Default|GetSquadMembers)
    (Class|IBPRTS|HustleUnit(Message) _array_element)))

(event EventCancelHustle
  (for _array_element (Variables|Default|GetSquadMembers)
    (Class|IBPRTS|CancelHustle(Message) _array_element)))

(event EventToCover
  (params (TargetCover :type BP%20Unit%20Cover%20Object%20Reference))
  (CallFunction|SquadTakeCover TargetCover))

(event EventSetDestination
  (params (Add :type Boolean) (ToCover :type Boolean) (Destination :type Vector :default "0, 0, 0"))
  (if (not ToCover)
    (Default|SetDestination (Variables|Default|GetSquadLeader) Add ToCover Destination)
    (Utilities|FlowControl|Delay 0.2)
    (if (> (Variables|Default|GetSquadSize) 1)
      (if (> (Variables|Default|GetSquadSize) 2)
        (CallFunction|NormalSquadMovement Add false "0, 0, 0")
        (else
          (CallFunction|DuoSquadMovement Add false "0, 0, 0"))))))

(event EventLeaveCover
  (for _array_element (Variables|Default|GetSquadMembers)
    (Class|IBPRTS|LeaveCover(Message) _array_element)))

(fn ConstructionScript)

(fn HustleSquad
  (bind _squadmembers (Variables|Default|GetSquadMembers))
  (if false
    (for _array_element _squadmembers
      (Class|IBPRTS|HustleUnit(Message) _array_element))
    (else
      (for _array_element_2 _squadmembers
        (Class|IBPRTS|CancelHustle(Message) _array_element_2)))))

(fn ChangeSquadStance
  (bind _squadleader (Variables|Default|GetSquadLeader))
  (Utilities|IsValid _squadleader
    (:Is%20Valid
      (switch Utilities|FlowControl|Switch|SwitchonE_UnitPosition (Variables|/Game/Blueprints/Units/UnitBlueprints/BP_UnitBase.BP_UnitBase_C|GetStance _squadleader)
        (:NewEnumerator2
          (Variables|/Game/Blueprints/Units/UnitBlueprints/BP_UnitBase.BP_UnitBase_C|SetStance _squadleader "NewEnumerator3"))
        (:NewEnumerator4
          (Variables|/Game/Blueprints/Units/UnitBlueprints/BP_UnitBase.BP_UnitBase_C|SetStance _squadleader "NewEnumerator2"))
        (:NewEnumerator3
          (Variables|/Game/Blueprints/Units/UnitBlueprints/BP_UnitBase.BP_UnitBase_C|SetStance _squadleader "NewEnumerator4")))
      (for _array_element (Variables|Default|GetSquadMembers)
        (Variables|/Game/Blueprints/Units/UnitBlueprints/BP_UnitBase.BP_UnitBase_C|SetStance _array_element (Variables|/Game/Blueprints/Units/UnitBlueprints/BP_UnitBase.BP_UnitBase_C|GetStance _squadleader))))))

(fn DeselectAllSelected
  (bind _squadmembers (Variables|Default|GetSquadMembers))
  (for _array_element _squadmembers
    (Class|IBPRTS|Deselected(Message) _array_element))
  (Utilities|Array|Clear _squadmembers))

(fn DuoSquadMovement
  (params (Add :type Boolean) (ToCover :type Boolean) (Destination :type Vector))
  (bind _squadleader (Variables|Default|GetSquadLeader))
  (Default|SetUnitDestination (Utilities|Array|Get(acopy) (Variables|BP_Squad_C|GetSquadMembers (Variables|/Game/Blueprints/Units/UnitBlueprints/BP_UnitBase.BP_UnitBase_C|GetSquad _squadleader)) 1) Add false (+ (* (Math|Vector|GetRightVector (.rotation (Transformation|GetActorTransform _squadleader))) 1.5e+02) (Variables|/Game/Blueprints/Units/UnitBlueprints/BP_UnitBase.BP_UnitBase_C|GetCurrentDestination _squadleader))))

(fn NormalSquadMovement
  (params (Add :type Boolean) (ToCover :type Boolean) (Destination :type Vector))
  (bind _squadleader (Variables|Default|GetSquadLeader))
  (bind _currentdestination (Variables|/Game/Blueprints/Units/UnitBlueprints/BP_UnitBase.BP_UnitBase_C|GetCurrentDestination _squadleader))
  (for (_array_element _array_index) (Variables|Default|GetSquadMembers)
    (if (!= _array_index 0)
      (bind _output_get (Variables|Default|SettempPosition (+ (Transformation|GetWorldLocation (Variables|/Script/Engine.Character|GetMesh _array_element)) (- _currentdestination (Transformation|GetWorldLocation (Variables|/Script/Engine.Character|GetMesh _squadleader))))))
      (if (< (Math|Vector|Distance(Vector) (+ (Transformation|GetWorldLocation (Variables|/Script/Engine.Character|GetMesh _array_element)) (- _currentdestination (Transformation|GetWorldLocation (Variables|/Script/Engine.Character|GetMesh _squadleader)))) _currentdestination) 1e+03)
        (Development|PrintString "In Range")
        (Default|SetUnitDestination _array_element Add false _output_get)
        (else
          (Development|PrintString "Out of Range")
          (Default|SetUnitDestination _array_element Add false (+ (* (- _currentdestination (+ (Transformation|GetWorldLocation (Variables|/Script/Engine.Character|GetMesh _array_element)) (- _currentdestination (Transformation|GetWorldLocation (Variables|/Script/Engine.Character|GetMesh _squadleader))))) (Math|Random|RandomFloatinRange 0.7 0.9)) _output_get)))))))

(fn RemovefromSquad
  (params (UnitToRemove :type BP%20Unit%20Base%20Object%20Reference))
  (bind _squadmembers (Variables|Default|GetSquadMembers))
  (Utilities|Array|RemoveItem _squadmembers UnitToRemove)
  (bind _output_get (Variables|Default|SetSquadSize (Utilities|Array|Length _squadmembers)))
  (if (> _output_get 0)
    (Utilities|IsValid (Variables|Default|GetSquadLeader)
      (:Is%20Not%20Valid
        (CallFunction|SetLeader)))
    (else
      (Actor|DestroyActor)
      (Development|PrintString "Squad Delted"))))

(fn AddtoSquad
  (params (UnitToAdd :type BP%20Unit%20Base%20Object%20Reference))
  (bind _squadmembers (Variables|Default|GetSquadMembers))
  (if (== (Variables|/Game/Blueprints/Units/UnitBlueprints/BP_UnitBase.BP_UnitBase_C|GetSquad UnitToAdd) self)
    _
    (else
      (CallFunction|RemovefromSquad (Variables|/Game/Blueprints/Units/UnitBlueprints/BP_UnitBase.BP_UnitBase_C|GetSquad UnitToAdd) UnitToAdd)))
  (Utilities|Array|AddUnique _squadmembers UnitToAdd)
  (Variables|Default|SetSquadSize (Utilities|Array|Length _squadmembers))
  (Variables|/Game/Blueprints/Units/UnitBlueprints/BP_UnitBase.BP_UnitBase_C|SetSquad UnitToAdd self))

(fn IsUnitinSquad
  (params (Unit :type BP%20Unit%20Base%20Object%20Reference))
  (for _array_element (Variables|Default|GetSquadMembers)
    (if (== _array_element Unit)
      (return true)))
  (return false))

(fn SetLeader
  (Variables|Default|SetSquadLeader (Utilities|Array|Get(acopy) (Variables|Default|GetSquadMembers))))

(fn SquadIconPosition
  (for _array_element (Variables|Default|GetSquadMembers)
    (Variables|Default|SetIconPosition (+ (Variables|Default|GetIconPosition) (Transformation|GetWorldLocation (Variables|/Script/Engine.Character|GetMesh _array_element)))))
  (bind _output_get (Variables|Default|SetIconPosition (/ (Variables|Default|GetIconPosition) (Variables|Default|GetSquadSize))))
  (return _output_get))

(fn SquadTakeCover
  (params (Cover :type BP%20Unit%20Cover%20Object%20Reference))
  (bind _psquadcover (Variables|/Game/Blueprints/Cover/BP_UnitCover.BP_UnitCover_C|GetPSquadCover Cover))
  (Development|PrintString (Utilities|String|ToString(Integer) (Utilities|Array|Length _psquadcover)))
  (for (_array_element _array_index) _psquadcover
    (Utilities|IsValid (Utilities|Array|Get(acopy) (Variables|Default|GetSquadMembers) _array_index)
      (:Is%20Valid
        (Class|IBPRTS|ToCover(Message) (Utilities|Array|Get(acopy) (Variables|Default|GetSquadMembers) _array_index) _array_element)
        (Default|SetUnitDestination (Utilities|Array|Get(acopy) (Variables|Default|GetSquadMembers) _array_index) false true (Transformation|GetActorLocation _array_element))))))

(fn SquadAttack
  (params (ActorToTarget :type Actor%20Object%20Reference) (TargetLocation :type Vector))
  (for _array_element (Variables|Default|GetSquadMembers)
    (Default|AttackOrder _array_element ActorToTarget TargetLocation)))

(fn MemberDied
  (params (DeadOne :type BP%20Unit%20Base%20Object%20Reference))
  (bind _squadmembers (Variables|Default|GetSquadMembers))
  (Utilities|Array|RemoveItem _squadmembers DeadOne)
  (bind _result (Math|Integer|DecrementInt (Variables|Default|GetSquadSize))
    (:%20%20
      (Variables|Default|SetSquadSize _result)
      (if (<= (Utilities|Array|Length _squadmembers) 0)
        (Actor|DestroyActor)
        (else
          (CallFunction|SetLeader))))))

(fn GetTeam
  (return 0))