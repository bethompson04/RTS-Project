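; Base character for a selectable RTS unit with squad membership, cover, inventory interaction and weapon equipping.
; Each unit spawns its own one-member squad at start, and selection highlights the squad leader differently.
; Move orders go through the AI controller or a waypoint queue, and overlapping cover snaps the unit into a stance.
; Tick updates hustle stamina, advances waypoints, triggers in-range interactions and shows stance through mesh materials.
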(event EventBeginPlay
  (Components|SkeletalMesh|SetSkeletalMeshAsset (Variables|Character|GetMesh) (Variables|Default|GetStaticMesh))
  (Rendering|SetVisibility (Variables|Default|GetSelectionMesh) false false)
  (CallFunction|LoneWolf))

(event EventSetDestination
  (params (Add :type Boolean) (ToCover :type Boolean) (Destination :type Vector :default "0, 0, 0"))
  (Variables|Default|SetTakingCover ToCover)
  (CallFunction|SetUnitDestination Add ToCover Destination))

(event EventLeaveCover
  (Variables|Default|SetCover 0)
  (Variables|Default|SetTakingCover false)
  (Variables|Default|SetStance "NewEnumerator2"))

(event Collision|EventActorBeginOverlap
  (params (OtherActor :type Actor%20Object%20Reference))
  (if true
    (if (and (Actor|ActorHasTag OtherActor "Cover") (Variables|Default|GetTakingCover))
      (CallFunction|TakeCover))))

(event EventRemovedfromSquad
  (params (ToNewSquad :type Boolean))
  (if ToNewSquad
    (CallFunction|LoneWolf)))

(event EventHustleUnit
  (Variables|Default|SetIsHustling true)
  (Variables|/Script/Engine.CharacterMovementComponent|SetMaxWalkSpeed (Variables|Character|GetCharacterMovement) 6e+02)
  (Variables|Default|SetStance "NewEnumerator2"))

(event EventTick
  (params (DeltaSeconds :type Float%20%28single-precision%29))
  (bind _bp_inventorycomponent (Variables|Default|GetBP_InventoryComponent))
  (bind _mesh (Variables|Character|GetMesh))
  (bind _destinationsarray (Variables|Default|GetDestinationsArray))
  (Utilities|FlowControl|Sequence
    (:then_0
      (if (Variables|Default|GetIsHustling)
        (Variables|Default|SetStamina (- (Variables|Default|GetStamina) (* DeltaSeconds 2.0)))
        (elif (<= (Variables|Default|GetStamina) (Variables|Default|GetMaxStamina))
          (Variables|Default|SetStamina (+ (Variables|Default|GetStamina) DeltaSeconds)))))
    (:then_1
      (if (Utilities|Array|IsValidIndex _destinationsarray)
        (Variables|Default|SetCurrentDestination (Utilities|Array|Get(acopy) _destinationsarray))
        (if (< (Math|Vector|VectorLength (- (Transformation|GetActorLocation) (Variables|Default|GetCurrentDestination))) 1.2e+02)
          (CallFunction|CheckforNextDestination))))
    (:then_2
      (bind _targetactor (Variables|/Game/Blueprints/Inventory/BP_InventoryComponent.BP_InventoryComponent_C|GetTargetActor _bp_inventorycomponent)
        (:then
          (Development|PrintString (Utilities|String|ToString(Float) (Transformation|GetDistanceTo _targetactor self)))
          (if (<= (Transformation|GetDistanceTo _targetactor self) (Variables|Default|GetInteractRange))
            (Default|Interact _bp_inventorycomponent)
            (Default|UpdateInventory (CallFunction|GetRTSPlayer) false)))
        (:else)))
    (:then_3
      (switch Utilities|FlowControl|Switch|SwitchonE_UnitPosition (Variables|Default|GetStance)
        (:NewEnumerator0
          (Rendering|Material|SetMaterial _mesh 0 "/Engine/Tutorial/SubEditors/TutorialAssets/Character/TutorialTPP_Mat.TutorialTPP_Mat" :!label _label))
        (:NewEnumerator1
          (goto _label))
        (:NewEnumerator2
          (Rendering|Material|SetMaterial _mesh 0 "/AnimationSharing/AnimSharingBase.AnimSharingBase"))
        (:NewEnumerator3
          (Rendering|Material|SetMaterial _mesh 0 "/AnimationSharing/AnimSharingGreen.AnimSharingGreen"))
        (:NewEnumerator4
          (Rendering|Material|SetMaterial _mesh 0 "/AnimationSharing/AnimSharingRed.AnimSharingRed"))))))

(event MouseInput|EventActorBeginCursorOver
  (Rendering|SetVisibility (Variables|Default|GetSelectionMesh) true false))

(event MouseInput|EventActorEndCursorOver
  (if (not (Variables|Default|GetIsSelected))
    (Rendering|SetVisibility (Variables|Default|GetSelectionMesh) false false)))

(event EventDeSelected
  (CallFunction|Deselect))

(event EventCancelHustle
  (Variables|Default|SetIsHustling false)
  (Variables|/Script/Engine.CharacterMovementComponent|SetMaxWalkSpeed (Variables|Character|GetCharacterMovement) 3e+02))

(event EventSelected
  (CallFunction|Select))

(event EventToCover
  (params (TargetCover :type BP%20Unit%20Cover%20Object%20Reference))
  (Variables|Default|SetCover TargetCover)
  (Variables|Default|SetTakingCover true))

(fn ConstructionScript)

(fn Select
  (bind _selectionmesh (Variables|Default|GetSelectionMesh))
  (Variables|Default|SetIsSelected true)
  (Rendering|SetVisibility _selectionmesh true false)
  (if (== (Variables|/Game/Blueprints/Units/BP_Squad.BP_Squad_C|GetSquadLeader (Variables|Default|GetSquad)) self)
    (Rendering|Material|SetMaterial _selectionmesh 0 "/AnimationSharing/AnimSharingBlue.AnimSharingBlue")
    (else
      (Rendering|Material|SetMaterial _selectionmesh 0 "/AnimationSharing/AnimSharingBase.AnimSharingBase"))))

(fn Deselect
  (Variables|Default|SetIsSelected false)
  (Rendering|SetVisibility (Variables|Default|GetSelectionMesh) false false))

(fn SetUnitDestination
  (params (Add :type Boolean) (ToCover :type Boolean) (Destination :type Vector))
  (bind _destinationsarray (Variables|Default|GetDestinationsArray))
  (if Add
    (Utilities|Array|AddUnique _destinationsarray Destination)
    (Development|PrintText "Added Destination")
    (else
      (AI|Navigation|MovetoLocation (AI|GetAIController self) Destination 16.0 true true true true "/Script/AIModule.NavFilter_AIControllerDefault")
      (Utilities|Array|Clear _destinationsarray)
      (Utilities|Array|AddUnique _destinationsarray Destination)
      (Development|PrintText "Set Destination"))))

(fn CheckforNextDestination
  (bind _destinationsarray (Variables|Default|GetDestinationsArray))
  (if (Utilities|Array|IsValidIndex _destinationsarray)
    (Utilities|Array|RemoveIndex _destinationsarray)
    (if (Utilities|Array|IsValidIndex _destinationsarray)
      (CallFunction|SetUnitDestination false false (Utilities|Array|Get(acopy) _destinationsarray))
      (else
        (Variables|Default|SetIsHustling false)
        (Variables|/Script/Engine.CharacterMovementComponent|SetMaxWalkSpeed (Variables|Character|GetCharacterMovement) 3e+02)))))

(fn TakeCover
  (bind _cover (Variables|Default|GetCover))
  (Transformation|SetWorldTransform (Variables|Collision|GetCapsuleComponent) (Transformation|GetActorTransform _cover) false false)
  (switch Utilities|FlowControl|Switch|SwitchonE_CoverType (Variables|/Game/Blueprints/Cover/BP_UnitCover.BP_UnitCover_C|GetCoverType _cover)
    (:NewEnumerator0
      (Variables|Default|SetStance "NewEnumerator0"))
    (:NewEnumerator1
      (Variables|Default|SetStance "NewEnumerator1"))
    (:NewEnumerator2
      (Variables|Default|SetStance "NewEnumerator4")))
  (Development|PrintString "In Cover!"))

(fn LoneWolf
  (Utilities|IsValid (Variables|Default|GetSquad)
    (:Is%20Valid
      (Default|RemovefromSquad (Variables|Default|GetSquad) self))
    (:Is%20Not%20Valid
      _))
  (bind _returnvalue (Game|SpawnActorfromClass "/Game/Blueprints/Units/BP_Squad.BP_Squad_C" (Transformation|GetActorTransform) "Undefined" "MultiplyWithRoot" 0 0))
  (bind _output_get (Variables|Default|SetSquad _returnvalue))
  (Default|AddtoSquad _output_get self))

(fn UnitInteractwith
  (bind _bp_inventorycomponent (Variables|Default|GetBP_InventoryComponent))
  (bind _targetactor (Variables|/Game/Blueprints/Inventory/BP_InventoryComponent.BP_InventoryComponent_C|GetTargetActor _bp_inventorycomponent)
    (:then
      (Development|PrintText (Utilities|Text|FormatText "Interact with: {target}" 0))
      (if (> (Math|Vector|Distance(Vector) (Transformation|GetActorLocation _targetactor) (Transformation|GetActorLocation)) (Variables|/Game/Blueprints/Inventory/BP_InventoryComponent.BP_InventoryComponent_C|GetPickupRange _bp_inventorycomponent))
        (CallFunction|SetUnitDestination false false "0, 0, 0")))
    (:else)))

(fn SetInteractTarget
  (params (InteractTarget :type Actor%20Object%20Reference))
  (bind _output_get (Variables|/Game/Blueprints/Inventory/BP_InventoryComponent.BP_InventoryComponent_C|SetTargetActor (Variables|Default|GetBP_InventoryComponent) InteractTarget))
  (Class|BPIInteractInterface|Lookat(Message) _output_get))

(fn ReloadWeapon)

(fn UseItem)

(fn EquipItem
  (params (ItemToEquip :type BP%20Weapon%20Base%20Object%20Reference))
  (bind _output_get (Variables|Default|SetEquippedWeapon ItemToEquip))
  (Transformation|SetActorTransform _output_get (Transformation|GetWorldTransform (Variables|Default|GetWeaponTransform))))