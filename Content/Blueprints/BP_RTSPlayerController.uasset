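; Player controller for RTS-style mouse control of unit squads, handling selection, orders, camera focus and inventory UI.
; Cursor traces pick the SelectedSquad, with Shift editing membership, while drag-box input is forwarded to the HUD.
; Destination clicks become move, take-cover, attack or interact orders on that squad, with Shift passed as an add flag.
; A briefly opened gate detects double-clicks to make units hustle; debug keys print inventory and emit noise.
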(event Custom|UpdateInventory
  (params (SameUnit :type Boolean))
  (bind _selectedsquad (Variables|Default|GetSelectedSquad))
  (bind _squadleader (Variables|/Game/Blueprints/Units/BP_Squad.BP_Squad_C|GetSquadLeader _selectedsquad))
  (Utilities|IsValid _squadleader
    (:Is%20Valid
      (Default|UpdateInventory (Variables|Default|GetPlayerUI) (Variables|/Game/Blueprints/Units/Blueprints/BP_UnitBase.BP_UnitBase_C|GetBP_InventoryComponent _squadleader)))))

(event Input|EnhancedActionEvents|EnhancedInputActionIA_SelectUnit
  (params (ActionValue :type Boolean) (ElapsedSeconds :type Float%20%28double-precision%29) (TriggeredSeconds :type Float%20%28double-precision%29) (InputAction :type Input%20Action%20Object%20Reference :default "/Game/Input/IA_SelectUnit.IA_SelectUnit"))
  (bind (_clickstart _clicklocation) (CallFunction|GetMouseVector))
  (bind _outhit (Class|KismetSystemLibrary|LineTraceSinglebyProfile _clickstart _clicklocation "BlockAllDynamic" false 0 "None" true))
  (bind _asbp_unit_base (Utilities|Casting|CastToBP_UnitBase (.HitActor (Collision|BreakHitResult _outhit)))
    (:then
      (bind _output_get (Variables|Default|SetSelectedSquad (Variables|/Game/Blueprints/Units/Blueprints/BP_UnitBase.BP_UnitBase_C|GetSquad _asbp_unit_base)))
      (Utilities|IsValid _output_get
        (:Is%20Valid
          (if (Variables|Default|GetShiftDown)
            (bind _insquad (Default|IsUnitinSquad _output_get _asbp_unit_base))
            (if _insquad
              (Class|IBPRTS|Deselected(Message) _asbp_unit_base)
              (Default|LoneWolf _asbp_unit_base)
              (else
                (Class|IBPRTS|Selected(Message) _asbp_unit_base)
                (Default|AddtoSquad (Variables|Default|GetSelectedSquad) _asbp_unit_base)))
            (elif (> (Variables|/Game/Blueprints/Units/BP_Squad.BP_Squad_C|GetSquadSize _output_get) 1)
              (Variables|Default|SetSelectedSquad (Variables|/Game/Blueprints/Units/Blueprints/BP_UnitBase.BP_UnitBase_C|GetSquad _asbp_unit_base))
              (Default|LoneWolf _asbp_unit_base)
              (else
                (Class|IBPRTS|Selected(Message) (Variables|/Game/Blueprints/Units/Blueprints/BP_UnitBase.BP_UnitBase_C|GetSquad _asbp_unit_base)))))
          (CallFunction|UpdateInventory false)
          (Variables|Default|SetAttackCommand false))
        (:Is%20Not%20Valid
          (CallFunction|DeselectSquad :!label _label)
          (Variables|Default|SetAttackCommand false))))
    (:CastFailed
      (goto _label))))

(event Input|EnhancedActionEvents|EnhancedInputActionIA_SelectUnitBox
  (params (ActionValue :type Boolean) (ElapsedSeconds :type Float%20%28double-precision%29) (TriggeredSeconds :type Float%20%28double-precision%29) (InputAction :type Input%20Action%20Object%20Reference :default "/Game/Input/IA_SelectUnitBox.IA_SelectUnitBox"))
  (bind _returnvalue (HUD|GetHUD))
  (:Triggered
    (Class|IBPRTS|Held(Message) _returnvalue))
  (:Started
    (Variables|Default|SetSelectBoxActive true)
    (Class|IBPRTS|Pressed(Message) _returnvalue))
  (:Canceled
    (Variables|Default|SetSelectBoxActive false :!label _label)
    (Class|IBPRTS|Released(Message) _returnvalue))
  (:Completed
    (goto _label)))

(event Input|EnhancedActionEvents|EnhancedInputActionIA_SetUnitDestination
  (params (ActionValue :type Boolean) (ElapsedSeconds :type Float%20%28double-precision%29) (TriggeredSeconds :type Float%20%28double-precision%29) (InputAction :type Input%20Action%20Object%20Reference :default "/Game/Input/IA_SetUnitDestination.IA_SetUnitDestination"))
  (bind _selectedsquad (Variables|Default|GetSelectedSquad))
  (bind _squadleader (Variables|/Game/Blueprints/Units/BP_Squad.BP_Squad_C|GetSquadLeader _selectedsquad))
  (Variables|Default|SetUnitHustle false)
  (Utilities|FlowControl|Sequence
    (:then_0
      (Utilities|FlowControl|Gate true :!label _label
        (:Exit
          (Variables|Default|SetUnitHustle true))))
    (:then_1
      (goto _label Open))
    (:then_2
      (Utilities|FlowControl|Delay 0.25)
      (goto _label Close))
    (:then_3
      (CallFunction|HustleSelectedUnits)
      (bind (_clickstart _clicklocation) (CallFunction|GetMouseVector))
      (bind _outhit (Class|KismetSystemLibrary|LineTraceSinglebyProfile _clickstart _clicklocation "BlockAllDynamic" false 0 "None" true))
      (Utilities|IsValid (.HitActor (Collision|BreakHitResult _outhit))
        (:Is%20Valid
          (if (not (Actor|ActorHasTag (.HitActor (Collision|BreakHitResult _outhit)) "Interactive"))
            (if (and (not (Actor|ActorHasTag (.HitActor (Collision|BreakHitResult _outhit)) "Unit")) (not (Variables|Default|GetAttackCommand)))
              (bind _asbp_unit_cover (Utilities|Casting|CastToBP_UnitCover (.HitActor (Collision|BreakHitResult _outhit)))
                (:then
                  (if (not (Variables|/Game/Blueprints/Cover/BP_UnitCover.BP_UnitCover_C|GetOccupied _asbp_unit_cover))
                    (Development|PrintString "take cover")
                    (CallFunction|SetSquadDestination true (.Location (Collision|BreakHitResult _outhit)) _asbp_unit_cover)
                    (Variables|Default|SetAttackCommand false :!label _label_2)))
                (:CastFailed
                  (CallFunction|SetSquadDestination false (.Location (Collision|BreakHitResult _outhit)))
                  (goto _label_2)))
              (else
                (Development|PrintString (Utilities|String|ToString(Vector) (.Location (Collision|BreakHitResult _outhit))))
                (bind _asbp_unit_base (Utilities|Casting|CastToBP_UnitBase (.HitActor (Collision|BreakHitResult _outhit)))
                  (:then
                    _)
                  (:CastFailed
                    _))
                (Default|SquadAttack (Variables|Default|GetSelectedSquad) _asbp_unit_base (.Location (Collision|BreakHitResult _outhit)))))
            (else
              (Default|SetInteractTarget _squadleader (.HitActor (Collision|BreakHitResult _outhit)))
              (Default|UnitInteractwith _squadleader)
              (goto _label_2))))))))

(event Input|EnhancedActionEvents|EnhancedInputActionIA_ToggleInventory
  (params (ActionValue :type Boolean) (ElapsedSeconds :type Float%20%28double-precision%29) (TriggeredSeconds :type Float%20%28double-precision%29) (InputAction :type Input%20Action%20Object%20Reference :default "/Game/Input/IA_ToggleInventory.IA_ToggleInventory"))
  (if true
    (Default|InventoryToggle (Variables|Default|GetPlayerUI))))

(event Input|EnhancedActionEvents|EnhancedInputActionIA_ShiftDown
  (params (ActionValue :type Boolean) (ElapsedSeconds :type Float%20%28double-precision%29) (TriggeredSeconds :type Float%20%28double-precision%29) (InputAction :type Input%20Action%20Object%20Reference :default "/Game/Input/IA_ShiftDown.IA_ShiftDown"))
  (:Triggered
    (Variables|Default|SetShiftDown true))
  (:Completed
    (Variables|Default|SetShiftDown false)))

(event Input|EnhancedActionEvents|EnhancedInputActionIA_FocusUnits
  (params (ActionValue :type Boolean) (ElapsedSeconds :type Float%20%28double-precision%29) (TriggeredSeconds :type Float%20%28double-precision%29) (InputAction :type Input%20Action%20Object%20Reference :default "/Game/Input/IA_FocusUnits.IA_FocusUnits"))
  (bind _selectedsquad (Variables|Default|GetSelectedSquad))
  (Utilities|IsValid _selectedsquad
    (:Is%20Valid
      (CallFunction|FocusCamerato (Transformation|GetActorLocation (Variables|/Game/Blueprints/Units/BP_Squad.BP_Squad_C|GetSquadLeader _selectedsquad))))))

(event EventBeginPlay
  (bind _returnvalue (Game|GetPlayerController 0))
  (Class|TurnBasedBlueprintLibrary|GetMyPlayerIndex)
  (Input|AddMappingContext (PlayerController|LocalPlayerSubsystems|GetEnhancedInputLocalPlayerSubsystem _returnvalue) "/Game/Input/IMC_RTS.IMC_RTS" 0 "(bIgnoreAllPressedKeysUntilRelease=True,bForceImmediately=False,bNotifyUserSettings=False)")
  (Variables|/Script/Engine.PlayerController|SetbShowMouseCursor _returnvalue true)
  (Class|PlayerController|ClientSetHUD "/Game/Blueprints/UserInterface/BP_PlayerHUD.BP_PlayerHUD_C")
  (bind _returnvalue_2 (UserInterface|CreateWidget "/Game/Blueprints/UserInterface/WBP_PlayerUI.WBP_PlayerUI_C"))
  (bind _output_get (Variables|Default|SetPlayerUI _returnvalue_2))
  (UserInterface|Viewport|AddtoViewport _output_get 0)
  (Variables|Default|SetPlayerTag "Player0"))

(event EventTick
  (params (DeltaSeconds :type Float%20%28single-precision%29))
  (bind _selectedsquad (Variables|Default|GetSelectedSquad))
  (bind (_clickstart _clicklocation) (CallFunction|GetMouseVector))
  (bind (_outhit _returnvalue) (Collision|LineTraceByChannel _clickstart _clicklocation "TraceTypeQuery3" false 0 "None"))
  (Utilities|IsValid _selectedsquad
    (:Is%20Valid
      (Utilities|IsValid (Variables|/Game/Blueprints/Units/BP_Squad.BP_Squad_C|GetSquadLeader _selectedsquad)
        (:Is%20Valid
          (if _returnvalue
            (Variables|Default|SetInteractTarget (.HitActor (Collision|BreakHitResult _outhit)))
            (else
              (Variables|Default|SetInteractTarget 0))))))))

(event Input|KeyboardEvents|DebugKeyR
  (params (Key :type Key%20Structure :default "None") (ActionValue :type Input%20Action%20Value%20Structure))
  (:Pressed
    (bind (_clickstart _clicklocation) (CallFunction|GetMouseVector))
    (bind _outhit (Class|KismetSystemLibrary|LineTraceSinglebyProfile _clickstart _clicklocation "BlockAllDynamic" false 0 "ForDuration" true "(R=1.000000,G=0.000000,B=0.000000,A=1.000000)" "(R=0.000000,G=1.000000,B=0.000000,A=1.000000)" 1.0))
    (Class|AISenseHearing|ReportNoiseEvent (.Location (Collision|BreakHitResult _outhit)) 1.0 self 6e+03 "Unit")))

(event Input|KeyboardEvents|1
  (params (Key :type Key%20Structure :default "None"))
  (bind _selectedsquad (Variables|Default|GetSelectedSquad))
  (bind _squadleader (Variables|/Game/Blueprints/Units/BP_Squad.BP_Squad_C|GetSquadLeader _selectedsquad))
  (bind _bp_inventorycomponent (Variables|/Game/Blueprints/Units/Blueprints/BP_UnitBase.BP_UnitBase_C|GetBP_InventoryComponent _squadleader))
  (:Pressed
    (Utilities|IsValid _bp_inventorycomponent
      (:Is%20Valid
        (Default|DEBUGPrintContents _bp_inventorycomponent)))))

(fn ConstructionScript)

(fn GetMouseVector
  (bind _returnvalue (Game|GetPlayerController 0))
  (bind (_worldlocation _worlddirection) (Game|Player|ConvertMouseLocationToWorldSpace _returnvalue))
  (return _worldlocation (+ _worldlocation (* _worlddirection 5e+03))))

(fn DeselectSquad
  (Class|IBPRTS|Deselected(Message) (Variables|Default|GetSelectedSquad))
  (Variables|Default|SetSelectedSquad 0))

(fn SetSquadDestination
  (params (ToCover :type Boolean) (Destination :type Vector) (CoverActor :type BP%20Unit%20Cover%20Object%20Reference))
  (bind _selectedsquad (Variables|Default|GetSelectedSquad))
  (if ToCover
    (Class|IBPRTS|ToCover(Message) _selectedsquad CoverActor)
    (Class|IBPRTS|SetDestination(Message) _selectedsquad (Variables|Default|GetShiftDown) ToCover Destination)
    (else
      (Class|IBPRTS|LeaveCover(Message) _selectedsquad)
      (Class|IBPRTS|SetDestination(Message) _selectedsquad (Variables|Default|GetShiftDown) ToCover Destination))))

(fn HustleSelectedUnits
  (bind _selectedsquad (Variables|Default|GetSelectedSquad))
  (if (Variables|Default|GetUnitHustle)
    (Class|IBPRTS|HustleUnit(Message) _selectedsquad)
    (else
      (Class|IBPRTS|CancelHustle(Message) _selectedsquad))))

(fn Interactwith)