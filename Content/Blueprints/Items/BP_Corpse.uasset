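; Corpse actor that recreates a dead character's mesh, armor and death pose, and holds its item contents in an inventory component.
; BeginPlay applies the corpse mesh, contents and per-slot armor meshes, then EquipArmor snaps each piece to its body socket and attaches it.
; DeathStance selects a non-looping standing, prone or crouched death animation, with other stances sharing the standing or crouched one.
; The HIghlight event is empty; its outline overlay logic is disconnected.
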(event EventBeginPlay
  (bind _mesh (Variables|Default|GetMesh))
  (Utilities|FlowControl|Sequence
    (:then_0
      (Components|SkeletalMesh|SetSkeletalMeshAsset (Variables|Default|GetMesh) (Variables|Default|GetCorpseMesh))
      (Variables|/Game/Blueprints/Inventory/BP_InventoryComponent.BP_InventoryComponent_C|SetContents (Variables|Default|GetBP_InventoryComponent) (Variables|Default|GetCorpseContents)))
    (:then_1
      (Components|StaticMesh|SetStaticMesh (Variables|Default|GetHelmetMesh) (Variables|Default|GetHelmetArmor))
      (Components|StaticMesh|SetStaticMesh (Variables|Default|GetChestMesh) (Variables|Default|GetChestArmor))
      (Components|StaticMesh|SetStaticMesh (Variables|Default|GetLShoulderMesh) (Variables|Default|GetLShoulderArmor))
      (Components|StaticMesh|SetStaticMesh (Variables|Default|GetRShoulderMesh) (Variables|Default|GetRShoulderArmor))
      (Components|StaticMesh|SetStaticMesh (Variables|Default|GetBeltMesh) (Variables|Default|GetBeltArmor))
      (Components|StaticMesh|SetStaticMesh (Variables|Default|GetLArmMesh) (Variables|Default|GetLArmArmor))
      (Components|StaticMesh|SetStaticMesh (Variables|Default|GetRArmMesh) (Variables|Default|GetRArmArmor))
      (Components|StaticMesh|SetStaticMesh (Variables|Default|GetLThighMesh) (Variables|Default|GetLThighArmor))
      (Components|StaticMesh|SetStaticMesh (Variables|Default|GetRThighMesh) (Variables|Default|GetRThighArmor))
      (Components|StaticMesh|SetStaticMesh (Variables|Default|GetLLegMesh) (Variables|Default|GetLLegArmor))
      (Components|StaticMesh|SetStaticMesh (Variables|Default|GetRLegMesh) (Variables|Default|GetRLegArmor))
      (CallFunction|EquipArmor))
    (:then_2
      (switch Utilities|FlowControl|Switch|SwitchonE_UnitPosition (Variables|Default|GetDeathStance)
        (:NewEnumerator2
          (Components|Animation|PlayAnimation _mesh "/Game/Assets/Models/Units/0StandDead.0StandDead" false :!label _label))
        (:NewEnumerator4
          (Components|Animation|PlayAnimation _mesh "/Game/Assets/Models/Units/0ProneDead.0ProneDead" false))
        (:NewEnumerator3
          (Components|Animation|PlayAnimation _mesh "/Game/Assets/Models/Units/0CrouchDead.0CrouchDead" false :!label _label_2))
        (:NewEnumerator0
          (goto _label))
        (:NewEnumerator1
          (goto _label_2))
        (:NewEnumerator7
          (goto _label))
        (:NewEnumerator8
          (goto _label))
        (:NewEnumerator6
          (goto _label))))))

(event EventHIghlight
  (params (doHighlight :type Boolean)))

(fn ConstructionScript
  (|CallParentFunction))

(fn EquipArmor
  (bind _beltmesh (Variables|Default|GetBeltMesh))
  (bind _mesh (Variables|Default|GetMesh))
  (bind _larmmesh (Variables|Default|GetLArmMesh))
  (bind _rarmmesh (Variables|Default|GetRArmMesh))
  (bind _mesh_2 (Variables|Default|GetMesh))
  (bind _helmetmesh (Variables|Default|GetHelmetMesh))
  (bind _chestmesh (Variables|Default|GetChestMesh))
  (bind _lshouldermesh (Variables|Default|GetLShoulderMesh))
  (bind _rshouldermesh (Variables|Default|GetRShoulderMesh))
  (bind _lthighmesh (Variables|Default|GetLThighMesh))
  (bind _llegmesh (Variables|Default|GetLLegMesh))
  (bind _rthighmesh (Variables|Default|GetRThighMesh))
  (bind _rlegmesh (Variables|Default|GetRLegMesh))
  (bind _mesh_3 (Variables|Default|GetMesh))
  (Utilities|FlowControl|Sequence
    (:then_0
      (Transformation|SetWorldTransform _helmetmesh (Transformation|GetSocketTransform (Variables|Default|GetMesh) "HelmetSocket" "RTS_World") false true)
      (Transformation|AttachComponentToComponent _helmetmesh _mesh_2 "HelmetSocket" "KeepWorld" "KeepWorld" "KeepWorld" true)
      (Transformation|SetWorldTransform _chestmesh (Transformation|GetSocketTransform (Variables|Default|GetMesh) "ChestSocket" "RTS_World") false true)
      (Transformation|AttachComponentToComponent _chestmesh _mesh_2 "ChestSocket" "KeepWorld" "KeepWorld" "KeepWorld" true)
      (Transformation|SetWorldTransform _lshouldermesh (Transformation|GetSocketTransform (Variables|Default|GetMesh) "LShoulderSocket" "RTS_World") false true)
      (Transformation|AttachComponentToComponent _lshouldermesh _mesh_2 "LShoulderSocket" "KeepWorld" "KeepWorld" "KeepWorld" true)
      (Transformation|SetWorldTransform _rshouldermesh (Transformation|GetSocketTransform (Variables|Default|GetMesh) "RShoulderSocket" "RTS_World") false true)
      (Transformation|AttachComponentToComponent _rshouldermesh _mesh_2 "RShoulderSocket" "KeepWorld" "KeepWorld" "KeepWorld" true))
    (:then_1
      (Transformation|SetWorldTransform _beltmesh (Transformation|GetSocketTransform (Variables|Default|GetMesh) "HipsSocket" "RTS_World") false true)
      (Transformation|AttachComponentToComponent _beltmesh _mesh_3 "HipsSocket" "KeepWorld" "KeepWorld" "KeepWorld" true)
      (Transformation|SetWorldTransform _larmmesh (Transformation|GetSocketTransform (Variables|Default|GetMesh) "LArmSocket" "RTS_World") false true)
      (Transformation|AttachComponentToComponent _larmmesh _mesh_3 "LArmSocket" "KeepWorld" "KeepWorld" "KeepWorld" true)
      (Transformation|SetWorldTransform _rarmmesh (Transformation|GetSocketTransform (Variables|Default|GetMesh) "RArmSocket" "RTS_World") false true)
      (Transformation|AttachComponentToComponent _rarmmesh _mesh_3 "RArmSocket" "KeepWorld" "KeepWorld" "KeepWorld" true))
    (:then_2
      (Transformation|SetWorldTransform _lthighmesh (Transformation|GetSocketTransform (Variables|Default|GetMesh) "LThighSocket" "RTS_World") false true)
      (Transformation|AttachComponentToComponent _lthighmesh _mesh "LThighSocket" "KeepWorld" "KeepWorld" "KeepWorld" true)
      (Transformation|SetWorldTransform _llegmesh (Transformation|GetSocketTransform (Variables|Default|GetMesh) "LLegSocket" "RTS_World") false true)
      (Transformation|AttachComponentToComponent _llegmesh _mesh "LLegSocket" "KeepWorld" "KeepWorld" "KeepWorld" true)
      (Transformation|SetWorldTransform _rthighmesh (Transformation|GetSocketTransform (Variables|Default|GetMesh) "RThighSocket" "RTS_World") false true)
      (Transformation|AttachComponentToComponent _rthighmesh _mesh "RThighSocket" "KeepWorld" "KeepWorld" "KeepWorld" true)
      (Transformation|SetWorldTransform _rlegmesh (Transformation|GetSocketTransform (Variables|Default|GetMesh) "RLegSocket" "RTS_World") false true)
      (Transformation|AttachComponentToComponent _rlegmesh _mesh "RLegSocket" "KeepWorld" "KeepWorld" "KeepWorld" true))))