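; BP_InteractableDoor is an interactable door that slides its static mesh vertically when used.
; UseEvent calls the parent implementation and passes its result to Open/Close as the open state.
; Open/Close instantly offsets the mesh's world location a fixed distance up to open or down to close, with no interpolation.
; Disconnected SetRelativeLocation and SetActive nodes remain in that function, and the default event nodes are disabled.
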(event EventBeginPlay
  (|CallParentFunction) ; This node is disabled and will not be called.\nDrag off pins to build functionality.
)

(event Collision|EventActorBeginOverlap
  (params (OtherActor :type Actor%20Object%20Reference))
  (|CallParentFunction OtherActor) ; This node is disabled and will not be called.\nDrag off pins to build functionality.
)

(event EventTick
  (params (DeltaSeconds :type Float%20%28single-precision%29))
  (|CallParentFunction DeltaSeconds) ; This node is disabled and will not be called.\nDrag off pins to build functionality.
)

(fn ConstructionScript
  (|CallParentFunction))

(fn UseEvent
  (bind _output_get (|CallParentFunction))
  (CallFunction|Open/Close _output_get))

(fn Open/Close
  (params (IsOpen :type Boolean))
  (bind _staticmesh (Variables|Default|GetStaticMesh))
  (bind _returnvalue (Transformation|GetWorldLocation _staticmesh))
  (if IsOpen
    (Transformation|SetWorldLocation _staticmesh (Math|Vector|MakeVector (.x _returnvalue) (.y _returnvalue) (+ (.z _returnvalue) 3e+02)) false false)
    (else
      (Transformation|SetWorldLocation _staticmesh (Math|Vector|MakeVector (.x _returnvalue) (.y _returnvalue) (- (.z _returnvalue) 3e+02)) false false)))
  (return))