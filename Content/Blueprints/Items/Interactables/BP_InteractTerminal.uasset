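; BP_InteractTerminal is an interactable terminal that can serve as the interact target of an RTS player objective.
; Its UseEvent override runs the parent logic while inactive, then checks whether it is the InteractTarget of the first objective type in player 0's ObjectiveTracker.
; On a match it destroys its LightActor, sets Active to block further use, and notifies the tracker of the interaction.
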(event EventBeginPlay
  (|CallParentFunction) ; This node is disabled and will not be called.\nDrag off pins to build functionality.
)

(event Collision|EventActorBeginOverlap
  (params (OtherActor :type Actor%20Object%20Reference))
  (|CallParentFunction OtherActor) ; This node is disabled and will not be called.\nDrag off pins to build functionality.
)

(event EventTick
  (params (DeltaSeconds :type Float%20%28single-precision%29))
  (|CallParentFunction DeltaSeconds) ; This node is disabled and will not be called.\nDrag off pins to build functionality.
)

(fn ConstructionScript
  (|CallParentFunction))

(fn UseEvent
  (bind _newparam (CallFunction|GetRTSPlayer))
  (bind _objectivetracker (Variables|/Game/Blueprints/BP_RTSPlayerController.BP_RTSPlayerController_C|GetObjectiveTracker _newparam))
  (if (not (Variables|Default|GetActive))
    (|CallParentFunction)
    (if (== self (.InteractTarget (Utilities|Struct|BreakF_ObjectiveStruct (Utilities|Array|Get(acopy) (Variables|/Game/Blueprints/BP_ObjectiveTracker.BP_ObjectiveTracker_C|GetObjectiveType _objectivetracker)))))
      (Actor|DestroyActor (Variables|Default|GetLightActor))
      (Variables|Default|SetActive true)
      (Default|CallObjectiveInteractedwith _objectivetracker))))