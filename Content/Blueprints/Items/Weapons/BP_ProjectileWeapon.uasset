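; Projectile weapon that fires an alien spit projectile from its barrel when the parent UseWeapon check passes.
; It extends the aim past the target and applies random accuracy-based rotation.
; An ammo table row and distance feed the damage passed to the spawned projectile, whose owner is the weapon.
; A debug-drawn line trace runs first but doesn't gate firing; the spit class is hardcoded, leaving the Projectile variable unused.
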(event EventBeginPlay
  (|CallParentFunction) ; This node is disabled and will not be called.\nDrag off pins to build functionality.
)

(event Collision|EventActorBeginOverlap
  (params (OtherActor :type Actor%20Object%20Reference))
  (|CallParentFunction OtherActor) ; This node is disabled and will not be called.\nDrag off pins to build functionality.
)

(event EventTick
  (params (DeltaSeconds :type Float%20%28single-precision%29))
  (|CallParentFunction DeltaSeconds) ; This node is disabled and will not be called.\nDrag off pins to build functionality.
)

(fn ConstructionScript
  (|CallParentFunction))

(fn UseWeapon
  (params (Target :type Vector :default "0, 0, 0"))
  (bind (_minaccuracy _maxaccuracy) (CallFunction|GetWeaponAccuracy))
  (bind (_minaccuracy_2 _maxaccuracy_2) (CallFunction|GetWeaponAccuracy))
  (bind _barrellocation (Variables|Default|GetBarrelLocation))
  (bind _ammostats (Variables|Default|GetAmmoStats))
  (bind _barrellocation_2 (Variables|Default|GetBarrelLocation))
  (bind _returnvalue (Transformation|GetWorldTransform _barrellocation))
  (bind _returnvalue_2 (Transformation|GetWorldLocation _barrellocation_2))
  (bind _returnvalue_3 (Math|Vector|GetRightVector _barrellocation_2))
  (bind _returnvalue_4 (Math|Random|RandomFloatinRange _minaccuracy_2 _maxaccuracy_2))
  (bind _returnvalue_5 (Math|Random|RandomFloatinRange _minaccuracy _maxaccuracy))
  (bind _returnvalue_6 (- Target _returnvalue_2))
  (bind _returnvalue_7 (Math|Vector|Normalize _returnvalue_6))
  (bind _returnvalue_8 (* _returnvalue_7 2.5e+03))
  (bind _returnvalue_9 (+ Target _returnvalue_8))
  (bind _returnvalue_10 (Math|Vector|RotateVectorAroundAxis _returnvalue_9 _returnvalue_4 _returnvalue_2))
  (bind _returnvalue_11 (Math|Vector|RotateVectorAroundAxis _returnvalue_10 _returnvalue_5 _returnvalue_3))
  (bind _success (|CallParentFunction Target))
  (if _success ; Can Fire, has target and ammo
    (bind _outhit (Collision|LineTraceByChannel _returnvalue_2 _returnvalue_11 "TraceTypeQuery1" false 0 "ForDuration" true "(R=1.000000,G=0.813819,B=0.058234,A=1.000000)" "(R=0.000000,G=1.000000,B=0.941990,A=1.000000)" 1.0))
    (bind _returnvalue_12 (Utilities|GetDataTableRow (.datatable _ammostats) (.rowname _ammostats))
      (:then
        (bind _returnvalue_13 (Game|SpawnActorfromClass "/Game/Blueprints/Items/Ammo/BP_AlienSpitProj.BP_AlienSpitProj_C" (Math|Transform|MakeTransform (.location _returnvalue) (Math|Rotator|FindLookatRotation _returnvalue_2 _returnvalue_11) (.scale _returnvalue)) "AlwaysSpawn" "MultiplyWithRoot" 0 (CallFunction|GetWeaponDamage (Math|Vector|Distance(Vector) _returnvalue_2 _returnvalue_11) (.AmmoRange (Utilities|Struct|BreakF_AmmoStruct _returnvalue_12)) (.AmmoDamage (Utilities|Struct|BreakF_AmmoStruct _returnvalue_12))) 0))
        (Variables|/Game/Blueprints/Items/Ammo/BP_AlienSpitProj.BP_AlienSpitProj_C|SetWeaponOwner _returnvalue_13 self)
        (return true)))
    (else
      (return false))))