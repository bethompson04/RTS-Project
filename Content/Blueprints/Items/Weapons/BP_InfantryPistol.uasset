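; BP_InfantryPistol is an infantry pistol weapon Blueprint that adds firing audio to its parent weapon class.
; Its UseWeapon override runs the parent logic on the target, plays one of two laser shot sounds at random at the barrel's world location, and returns the parent's result.
; The event graph and construction script add no logic of their own.
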(event EventBeginPlay
  (|CallParentFunction) ; This node is disabled and will not be called.\nDrag off pins to build functionality.
)

(event Collision|EventActorBeginOverlap
  (params (OtherActor :type Actor%20Object%20Reference))
  (|CallParentFunction OtherActor) ; This node is disabled and will not be called.\nDrag off pins to build functionality.
)

(event EventTick
  (params (DeltaSeconds :type Float%20%28single-precision%29))
  (|CallParentFunction DeltaSeconds) ; This node is disabled and will not be called.\nDrag off pins to build functionality.
)

(fn ConstructionScript
  (|CallParentFunction))

(fn UseWeapon
  (params (Target :type Vector :default "0, 0, 0"))
  (bind _barrellocation (Variables|Default|GetBarrelLocation))
  (bind _returnvalue (Transformation|GetWorldLocation _barrellocation))
  (bind _success (|CallParentFunction Target))
  (switch int (Math|Random|RandomIntegerinRange 0 1)
    (:Default
      _)
    (:0
      (Audio|PlaySoundatLocation "/Game/Assets/Sounds/LaserShot5.LaserShot5" _returnvalue "0, 0, 0" 1.0 1.0 0.0 0 0 0 0))
    (:1
      (Audio|PlaySoundatLocation "/Game/Assets/Sounds/LaserShot6.LaserShot6" _returnvalue "0, 0, 0" 1.0 1.0 0.0 0 0 0 0)))
  (return _success))