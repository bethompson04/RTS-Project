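; Hitscan laser weapon that overrides UseWeapon, firing only when the parent's check passes.
; It traces from the barrel to a point beyond the target, randomly rotated by weapon accuracy, and spawns colored Niagara beam and impact effects.
; Hit actors with BP_HealthComponent take damage from the ammo data-table row.
; Damage falloff uses the distance from the target to a randomized endpoint, not to the hit location.
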(event EventBeginPlay
  (|CallParentFunction) ; This node is disabled and will not be called.\nDrag off pins to build functionality.
)

(event Collision|EventActorBeginOverlap
  (params (OtherActor :type Actor%20Object%20Reference))
  (|CallParentFunction OtherActor) ; This node is disabled and will not be called.\nDrag off pins to build functionality.
)

(event EventTick
  (params (DeltaSeconds :type Float%20%28single-precision%29))
  (|CallParentFunction DeltaSeconds) ; This node is disabled and will not be called.\nDrag off pins to build functionality.
)

(fn ConstructionScript
  (|CallParentFunction))

(fn UseWeapon
  (params (Target :type Vector :default "0, 0, 0"))
  (bind (_minaccuracy _maxaccuracy) (CallFunction|GetWeaponAccuracy))
  (bind (_minaccuracy_2 _maxaccuracy_2) (CallFunction|GetWeaponAccuracy))
  (bind _ammostats (Variables|Default|GetAmmoStats))
  (bind _barrellocation (Variables|Default|GetBarrelLocation))
  (bind _returnvalue (Transformation|GetWorldLocation _barrellocation))
  (bind _returnvalue_2 (Math|Vector|GetRightVector _barrellocation))
  (bind _returnvalue_3 (Math|Random|RandomFloatinRange _minaccuracy_2 _maxaccuracy_2))
  (bind _returnvalue_4 (Math|Random|RandomFloatinRange _minaccuracy _maxaccuracy))
  (bind _returnvalue_5 (- Target _returnvalue))
  (bind _returnvalue_6 (Math|Vector|Normalize _returnvalue_5))
  (bind _returnvalue_7 (* _returnvalue_6 2.5e+03))
  (bind _returnvalue_8 (+ Target _returnvalue_7))
  (bind _returnvalue_9 (Math|Vector|RotateVectorAroundAxis _returnvalue_8 _returnvalue_3 _returnvalue))
  (bind _returnvalue_10 (Math|Vector|RotateVectorAroundAxis _returnvalue_9 _returnvalue_4 _returnvalue_2))
  (bind _success (|CallParentFunction Target))
  (if _success ; Can Fire, has target and ammo
    (bind _outhit (Collision|LineTraceByChannel _returnvalue _returnvalue_10 "TraceTypeQuery1" false 0 "None" true "(R=1.000000,G=0.813819,B=0.058234,A=1.000000)" "(R=0.000000,G=1.000000,B=0.941990,A=1.000000)" 1.0))
    (bind _returnvalue_11 (Niagara|SpawnSystematLocation "/Game/Assets/FX/NS_Laser.NS_Laser" _returnvalue))
    (Utilities|IsValid (.HitActor (Collision|BreakHitResult _outhit))
      (:Is%20Valid
        (Class|NiagaraComponent|SetVariablePosition _returnvalue_11 "BeamEnd" (.Location (Collision|BreakHitResult _outhit)))
        (bind _returnvalue_12 (Niagara|SpawnSystematLocation "/Game/Assets/FX/NS_LaserImpact.NS_LaserImpact" (.Location (Collision|BreakHitResult _outhit))))
        (Niagara|SetNiagaraVariable(LinearColor) _returnvalue_12 "ImpactColor" (Variables|Default|GetLaserColor)))
      (:Is%20Not%20Valid
        (Class|NiagaraComponent|SetVariablePosition _returnvalue_11 "BeamEnd" _returnvalue_10)))
    (Effects|Components|ParticleSystem|SetColorParameter _returnvalue_11 "BeamColor" (Variables|Default|GetLaserColor))
    (Utilities|IsValid (Actor|GetComponentbyClass (.HitActor (Collision|BreakHitResult _outhit)) "/Game/Blueprints/Units/BP_HealthComponent.BP_HealthComponent_C")
      (:Is%20Valid
        (bind _returnvalue_13 (Utilities|GetDataTableRow (.datatable _ammostats) (.rowname _ammostats))
          (:then
            (Development|PrintText (Utilities|Text|FormatText "Hit Damage: {Damage}" (CallFunction|GetWeaponDamage (Math|Vector|Distance(Vector) Target _returnvalue_10) (.AmmoRange (Utilities|Struct|BreakF_AmmoStruct _returnvalue_13)) (.AmmoDamage (Utilities|Struct|BreakF_AmmoStruct _returnvalue_13)))))
            (Default|TakeDamage (Actor|GetComponentbyClass (.HitActor (Collision|BreakHitResult _outhit)) "/Game/Blueprints/Units/BP_HealthComponent.BP_HealthComponent_C") (CallFunction|GetWeaponDamage (Math|Vector|Distance(Vector) Target _returnvalue_10) (.AmmoRange (Utilities|Struct|BreakF_AmmoStruct _returnvalue_13)) (.AmmoDamage (Utilities|Struct|BreakF_AmmoStruct _returnvalue_13))) (Variables|Default|GetUnitOwner))
            (return true)))))
    (else
      (return false))))