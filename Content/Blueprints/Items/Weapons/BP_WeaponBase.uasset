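; Base weapon Blueprint for units, handling firing, ammo, reloading and damage calculation.
; UseWeapon moves the owner closer when the target is out of range; otherwise it spends ammo, updates the inventory slot, fires a debug-drawn trace and makes noise for AI hearing.
; An empty magazine tells the owning unit to reload.
; Helper functions return the accuracy spread and distance-falloff damage, but the trace itself applies no damage.
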(event Custom|MagEmpty
  (bind _unitowner (Variables|Default|GetUnitOwner))
  (Utilities|IsValid _unitowner
    (:Is%20Valid
      (Default|ReloadUnitWeapon _unitowner))))

(event EventBeginPlay
  (Variables|/Game/Blueprints/Inventory/BP_ItemDataComponent.BP_ItemDataComponent_C|SetAmmo (Variables|Default|GetBP_ItemDataComponent) (Variables|Default|GetMagAmmo)))

(event Collision|EventActorBeginOverlap
  (params (OtherActor :type Actor%20Object%20Reference)))

(event EventTick
  (params (DeltaSeconds :type Float%20%28single-precision%29)))

(fn ConstructionScript)

(fn UseWeapon
  (params (Target :type Vector))
  (bind _unitowner (Variables|Default|GetUnitOwner))
  (bind _unitowner_2 (Variables|Default|GetUnitOwner))
  (bind _unitowner_3 (Variables|Default|GetUnitOwner))
  (bind _bp_itemdatacomponent (Variables|Default|GetBP_ItemDataComponent))
  (bind _barrellocation (Variables|Default|GetBarrelLocation))
  (bind _returnvalue (Transformation|GetWorldLocation _barrellocation))
  (bind _returnvalue_2 (Transformation|GetActorLocation _unitowner_3))
  (if (> (Math|Vector|Distance(Vector) Target (Transformation|GetActorLocation (Variables|Default|GetUnitOwner))) (Variables|Default|GetRange)) ; If distance to target is greater than Weapon's effective range
    (Default|SetUnitDestination _unitowner false false (+ _returnvalue_2 (* (Math|Vector|Normalize (- Target _returnvalue_2)) (- (Math|Vector|Distance(Vector) _returnvalue_2 Target) (- (Variables|Default|GetRange) 1e+02)))))
    (return false)
    (elif (> (Variables|/Game/Blueprints/Inventory/BP_ItemDataComponent.BP_ItemDataComponent_C|GetAmmo _bp_itemdatacomponent) 0)
      (bind _result (Math|Integer|DecrementInt (Variables|/Game/Blueprints/Inventory/BP_ItemDataComponent.BP_ItemDataComponent_C|GetAmmo _bp_itemdatacomponent))
        (:%20%20
          (bind _output_get (Variables|/Game/Blueprints/Inventory/BP_ItemDataComponent.BP_ItemDataComponent_C|SetAmmo _bp_itemdatacomponent _result))
          (Default|UpdateSlotAmmo (Variables|/Game/Blueprints/Units/UnitBlueprints/BP_UnitBase.BP_UnitBase_C|GetBP_InventoryComponent _unitowner) (Variables|/Game/Blueprints/Inventory/BP_ItemDataComponent.BP_ItemDataComponent_C|GetInventoryIndex (Variables|Default|GetBP_ItemDataComponent)) _output_get)
          (Collision|LineTraceByChannel _returnvalue (+ Target (* (Math|Vector|Normalize (- Target _returnvalue)) 2.5e+03)) "TraceTypeQuery1" false 0 "ForDuration" true "(R=1.000000,G=0.000000,B=0.000000,A=1.000000)" "(R=0.000000,G=1.000000,B=0.000000,A=1.000000)" 1.0)
          (Class|Actor|MakeNoise 1.0 _unitowner_2 (Transformation|GetActorLocation _unitowner_2) 6e+03 "Sound")
          (return true)))
      (else
        (CallFunction|MagEmpty)
        (return false)))))

(fn Reload
  (params (AmountCanReload :type Integer))
  (bind _bp_itemdatacomponent (Variables|Default|GetBP_ItemDataComponent))
  (if (< (Variables|/Game/Blueprints/Inventory/BP_ItemDataComponent.BP_ItemDataComponent_C|GetAmmo _bp_itemdatacomponent) (Variables|Default|GetMagSize))
    (Variables|/Game/Blueprints/Inventory/BP_ItemDataComponent.BP_ItemDataComponent_C|SetAmmo _bp_itemdatacomponent AmountCanReload)
    (return true)))

(fn SetWeaponOwner
  (params (Owner :type BP%20Unit%20Base%20Object%20Reference))
  (Variables|Default|SetUnitOwner Owner))

(fn GetWeaponAccuracy
  (return (* (Variables|Default|GetAccuracy) -1.0) (Variables|Default|GetAccuracy)))

(fn GetWeaponDamage
  (params (Distance :type Float%20%28double-precision%29) (Falloff :type Float%20%28double-precision%29) (AmmoDamage :type Float%20%28double-precision%29))
  (bind _damage (Variables|Default|GetDamage))
  (bind _returnvalue (+ AmmoDamage _damage))
  (if (> Distance Falloff)
    (bind _output_get (LocalVariables|SetLocal_Damage (- _returnvalue (* (/ Distance Falloff) (Math|Conversions|ToFloat(Integer) (.ReturnValue (Math|Float|Division(WholeandRemainder) Distance Falloff)))))))
    (return _output_get)
    (else
      (bind _output_get_2 (LocalVariables|SetLocal_Damage _returnvalue))
      (return _output_get_2))))