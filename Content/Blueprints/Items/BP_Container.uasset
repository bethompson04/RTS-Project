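; Item container that shows its inventory in the RTS player's UI when a unit interacts with it.
; Interaction stores the unit and, if not already open, sets IsOpen and passes the inventory component to PlayerUI.
; Tick removes all top-level container inventory widgets, found by class search, while that unit is beyond the component's pickup range.
; This graph never resets IsOpen or the stored unit.
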(event EventTick
  (params (DeltaSeconds :type Float%20%28single-precision%29))
  (bind _interactingunit (Variables|Default|GetInteractingUnit))
  (Utilities|IsValid _interactingunit
    (:Is%20Valid
      (if (> (Transformation|GetDistanceTo _interactingunit) (Variables|/Game/Blueprints/Inventory/BP_InventoryComponent.BP_InventoryComponent_C|GetPickupRange (Variables|Default|GetBP_InventoryComponent)))
        (bind _foundwidgets (Widget|GetAllWidgetsOfClass "/Game/Blueprints/Inventory/UI/WBP_ContainerInventory.WBP_ContainerInventory_C" true)) ; oh god
        (for _array_element _foundwidgets
          (Default|RemoveContainerInventory _array_element))))))

(event EventInteractwith
  (params (InteractingUnit :type BP%20Unit%20Base%20Object%20Reference))
  (Variables|Default|SetInteractingUnit InteractingUnit)
  (if (not (Variables|Default|GetIsOpen))
    (Variables|Default|SetIsOpen true)
    (Default|ShowContainer (Variables|/Game/Blueprints/BP_RTSPlayerController.BP_RTSPlayerController_C|GetPlayerUI (CallFunction|GetRTSPlayer)) (Variables|Default|GetBP_InventoryComponent))))

(fn ConstructionScript)