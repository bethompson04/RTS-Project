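; BP_Medkit is a medkit item Blueprint that can be highlighted and used by a unit.
; The Highlight event toggles an interaction outline by setting or clearing the static mesh's overlay material.
; UseItem extends the parent implementation, then calls MedkitUse on the using owner, with heal rate and duration both passed as zero.
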(event EventBeginPlay
  (|CallParentFunction) ; This node is disabled and will not be called.\nDrag off pins to build functionality.
)

(event Collision|EventActorBeginOverlap
  (params (OtherActor :type Actor%20Object%20Reference))
  (|CallParentFunction OtherActor) ; This node is disabled and will not be called.\nDrag off pins to build functionality.
)

(event EventTick
  (params (DeltaSeconds :type Float%20%28single-precision%29))
  (|CallParentFunction DeltaSeconds) ; This node is disabled and will not be called.\nDrag off pins to build functionality.
)

(event EventHIghlight
  (params (doHighlight :type Boolean))
  (bind _staticmesh (Variables|Default|GetStaticMesh))
  (if doHighlight
    (Rendering|Material|SetOverlayMaterial _staticmesh "/Game/Assets/Materials/M_InteractOutline.M_InteractOutline" :!class /Script/Engine.MeshComponent)
    (else
      (Rendering|Material|SetOverlayMaterial _staticmesh 0 :!class /Script/Engine.MeshComponent))))

(fn ConstructionScript
  (|CallParentFunction))

(fn UseItem
  (params (OwnerUsing :type BP%20Unit%20Base%20Object%20Reference))
  (|CallParentFunction OwnerUsing)
  (CallFunction|MedkitUse OwnerUsing 0.0 0.0))