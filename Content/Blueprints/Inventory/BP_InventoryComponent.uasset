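; Inventory component for BP_UnitBase owners that stores fixed-size slots of item ID, quantity and ammo.
; Adding fills partial stacks before empty slots using DT_ItemData limits, while transfers between inventories merge matching items or swap slots.
; Using items consumes them or toggles equipped weapons with slot ammo, and non-consumed removals spawn pickups ahead of the owner.
; Server events handle interaction, transfers and drops, and MC_Update broadcasts changes from removals and transfers.
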(event Custom|Server_Interact
  (params (Target :type Actor%20Object%20Reference))
  (bind _returnvalue (Actor|GetComponentbyClass Target "/Game/Blueprints/Inventory/BP_ItemDataComponent.BP_ItemDataComponent_C"))
  (bind _returnvalue_2 (Components|GetOwner))
  (bind _asbp_unit_base (Utilities|Casting|CastToBP_UnitBase _returnvalue_2))
  (Utilities|IsValid _returnvalue
    (:Is%20Valid
      (Class|BPIInteractInterface|Interactwith(Message) _returnvalue _asbp_unit_base))
    (:Is%20Not%20Valid
      (Actor|SetOwner Target (Pawn|GetController _asbp_unit_base))
      (CallFunction|OnLocalInteract Target _asbp_unit_base))))

(event Custom|Interact
  (bind _targetactor (Variables|Default|GetTargetActor)
    (:then
      (CallFunction|ServerInteract _targetactor))
    (:else)))

(event Custom|MC_Update
  (Default|CallOnInventoryUpdated))

(event Custom|SERVER_TransferSlots
  (params (SourceIndex :type Integer) (SourceInventory :type BP%20Inventory%20Component%20Object%20Reference) (DestinationIndex :type Integer))
  (CallFunction|TransferSlots SourceIndex SourceInventory DestinationIndex))

(event Custom|OnLocalInteract
  (params (TargetActor :type Actor%20Object%20Reference) (Interactor :type Actor%20Object%20Reference))
  (Class|BPIInteractInterface|Interactwith(Message) TargetActor (.AsBP%20Unit%20Base (Utilities|Casting|CastToBP_UnitBase Interactor))))

(event Custom|SERVER_REMOVE
  (params (Index :type Integer) (IsCosumed :type Boolean))
  (if IsCosumed
    _))

(event Custom|SERVER_DropItem
  (params (ItemID :type Name) (Quantity :type Integer))
  (bind _returnvalue (Game|SpawnActorfromClass (.ItemClass (Utilities|Struct|BreakF_ItemStruct (CallFunction|GetItemData ItemID))) (Math|Transform|MakeTransform (CallFunction|GetDropLocation) "0, 0, 0" "1.000000,1.000000,1.000000") "Undefined" "MultiplyWithRoot" 0 0))
  (Variables|/Game/Blueprints/Inventory/BP_ItemDataComponent.BP_ItemDataComponent_C|SetQuantity (Actor|GetComponentbyClass _returnvalue "/Game/Blueprints/Inventory/BP_ItemDataComponent.BP_ItemDataComponent_C") Quantity))

(event Custom|UpdateSlotAmmo
  (params (Index :type Integer) (NewCount :type Integer))
  (bind _contents (Variables|Default|GetContents))
  (bind _output (Utilities|Array|Get(acopy) _contents Index))
  (bind (_itemid _quantity) (Utilities|Struct|BreakF_SlotStruct _output))
  (Utilities|Array|SetArrayElem _contents Index (Utilities|Struct|MakeF_SlotStruct _itemid _quantity NewCount)))

(event EventBeginPlay
  (Utilities|Array|Resize (Variables|Default|GetContents) (Variables|Default|GetInventorySize)))

(fn AddtoInventory
  (params (ItemID :type Name) (Quantity :type Integer) (Ammo :type Integer))
  (bind _output_get (LocalVariables|SetL_QuantityRemaining Quantity))
  (while (and (> _output_get 0) (not (LocalVariables|GetL_HasFailed)))
    (bind (_index _foundslot) (CallFunction|FindOpenSlot ItemID))
    (if _foundslot
      (CallFunction|AddtoStack _index 1)
      (Math|Integer|DecrementInt (LocalVariables|GetL_QuantityRemaining))
      (elif (.HasEmptySlot (CallFunction|FindAvailableEmptySlots))
        (bind (_success _index_2) (CallFunction|CreateNewStack ItemID 1 Ammo))
        (if _success
          (Math|Integer|DecrementInt (LocalVariables|GetL_QuantityRemaining))
          (else
            (LocalVariables|SetL_HasFailed true :!label _label)))
        (else
          (goto _label)))))
  (return (not (LocalVariables|GetL_HasFailed)) (LocalVariables|GetL_QuantityRemaining) _index_2))

(fn RemovefromInventory
  (params (Index :type Integer) (IsConsumed :type Boolean) (QuantityRemoved :type Integer))
  (bind _contents (Variables|Default|GetContents))
  (bind _contents_2 (Variables|Default|GetContents))
  (bind _output (Utilities|Array|Get(acopy) _contents Index))
  (LocalVariables|SetLocal_ItemID (.itemid _output))
  (LocalVariables|SetLocal_Quantity (.quantity _output))
  (Utilities|FlowControl|Sequence
    (:then_0
      (if IsConsumed
        (bind _output_get (LocalVariables|SetLocal_Quantity (- (LocalVariables|GetLocal_Quantity) QuantityRemoved)))
        (Utilities|Array|SetArrayElem _contents_2 Index (Utilities|Struct|MakeF_SlotStruct (LocalVariables|GetLocal_ItemID) _output_get 0))
        (else
          (Utilities|Array|SetArrayElem _contents_2 Index (Utilities|Struct|MakeF_SlotStruct "None" 0 0))
          (CallFunction|SERVERDropItem (LocalVariables|GetLocal_ItemID) (LocalVariables|GetLocal_Quantity)))))
    (:then_1
      (CallFunction|MCUpdate))))

(fn FindOpenSlot
  (params (ItemID :type Name))
  (for (_array_element _array_index) (Variables|Default|GetContents)
    (if (== (.ItemID (Utilities|Struct|BreakF_SlotStruct _array_element)) ItemID)
      (if (< (.Quantity (Utilities|Struct|BreakF_SlotStruct _array_element)) (CallFunction|GetMaxStackSize ItemID))
        (return _array_index true))))
  (return -1 false))

(fn GetMaxStackSize
  (params (ItemID :type Name))
  (bind _returnvalue (Utilities|GetDataTableRow "/Game/Blueprints/Items/DT_ItemData.DT_ItemData" ItemID)
    (:then
      (return (.StackSize (Utilities|Struct|BreakF_ItemStruct _returnvalue))))
    (:RowNotFound
      (return -1))))

(fn AddtoStack
  (params (Index :type Integer) (IncreaseQuantity :type Integer))
  (bind _contents (Variables|Default|GetContents))
  (bind _output (Utilities|Array|Get(acopy) _contents Index))
  (Utilities|Array|SetArrayElem _contents Index (Utilities|Struct|MakeF_SlotStruct (.itemid _output) (+ (.quantity _output) IncreaseQuantity))))

(fn FindAvailableEmptySlots
  (for (_array_element _array_index) (Variables|Default|GetContents)
    (if (== (.Quantity (Utilities|Struct|BreakF_SlotStruct _array_element)) 0)
      (return true _array_index)))
  (return false -1))

(fn CreateNewStack
  (params (ItemID :type Name) (Quantity :type Integer) (Ammo :type Integer))
  (bind (_hasemptyslot _emptyindex) (CallFunction|FindAvailableEmptySlots))
  (if _hasemptyslot
    (Utilities|Array|SetArrayElem (Variables|Default|GetContents) _emptyindex (Utilities|Struct|MakeF_SlotStruct ItemID Quantity Ammo))
    (return true _emptyindex)
    (else
      (return false -1))))

(fn DEBUGPrintContents
  (for (_array_element _array_index) (Variables|Default|GetContents)
    (if (> (.Quantity (Utilities|Struct|BreakF_SlotStruct _array_element)) 0)
      (Development|PrintString (Utilities|String|Append (Utilities|String|ToString(Integer) _array_index) ":" (Utilities|String|ToString(Name) (.ItemID (Utilities|Struct|BreakF_SlotStruct _array_element))) "=" (Utilities|String|ToString(Integer) (.Quantity (Utilities|Struct|BreakF_SlotStruct _array_element))) "Ammo:" (Utilities|String|ToString(Integer) (.Ammo (Utilities|Struct|BreakF_SlotStruct _array_element))))))))

(fn TransferSlots
  (params (SourceIndex :type Integer) (SourceInventory :type BP%20Inventory%20Component%20Object%20Reference) (DestinationIndex :type Integer))
  (LocalVariables|SetLocalSlotContent (Utilities|Array|Get(acopy) (Variables|BP_InventoryComponent_C|GetContents SourceInventory) SourceIndex))
  (if (not (< DestinationIndex 0))
    (if (== (.ItemID (Utilities|Struct|BreakF_SlotStruct (Utilities|Array|Get(acopy) (Variables|Default|GetContents) DestinationIndex))) (.ItemID (Utilities|Struct|BreakF_SlotStruct (LocalVariables|GetLocalSlotContent))))
      (Utilities|Array|SetArrayElem (Variables|BP_InventoryComponent_C|GetContents SourceInventory) SourceIndex (Utilities|Struct|MakeF_SlotStruct (select (> (Math|Integer|Clamp(Integer) (- (+ (.quantity (LocalVariables|GetLocalSlotContent)) (.quantity (Utilities|Array|Get(acopy) (Variables|Default|GetContents) DestinationIndex))) (CallFunction|GetMaxStackSize (.itemid (LocalVariables|GetLocalSlotContent)))) 0 (CallFunction|GetMaxStackSize (.itemid (LocalVariables|GetLocalSlotContent)))) 0) (.itemid (LocalVariables|GetLocalSlotContent)) "None") (Math|Integer|Clamp(Integer) (- (+ (.quantity (LocalVariables|GetLocalSlotContent)) (.quantity (Utilities|Array|Get(acopy) (Variables|Default|GetContents) DestinationIndex))) (CallFunction|GetMaxStackSize (.itemid (LocalVariables|GetLocalSlotContent)))) 0 (CallFunction|GetMaxStackSize (.itemid (LocalVariables|GetLocalSlotContent)))) 0))
      (Utilities|Array|SetArrayElem (Variables|Default|GetContents) DestinationIndex (Utilities|Struct|MakeF_SlotStruct (.itemid (LocalVariables|GetLocalSlotContent)) (Math|Integer|Clamp(Integer) (+ (.quantity (LocalVariables|GetLocalSlotContent)) (.quantity (Utilities|Array|Get(acopy) (Variables|Default|GetContents) DestinationIndex))) 0 (CallFunction|GetMaxStackSize (.itemid (LocalVariables|GetLocalSlotContent)))) 0))
      (CallFunction|MCUpdate)
      (CallFunction|MCUpdate SourceInventory)
      (else
        (Utilities|Array|SetArrayElem (Variables|BP_InventoryComponent_C|GetContents SourceInventory) SourceIndex (Utilities|Array|Get(acopy) (Variables|Default|GetContents) DestinationIndex))
        (Utilities|Array|SetArrayElem (Variables|Default|GetContents) DestinationIndex (LocalVariables|GetLocalSlotContent))
        (CallFunction|MCUpdate)
        (CallFunction|MCUpdate SourceInventory)))))

(fn GetItemData
  (params (ItemID :type Name))
  (bind _returnvalue (Utilities|GetDataTableRow "/Game/Blueprints/Items/DT_ItemData.DT_ItemData" ItemID)
    (:then
      (return _returnvalue))))

(fn GetDropLocation
  (bind _returnvalue (Components|GetOwner))
  (return (+ (Transformation|GetActorLocation _returnvalue) (* (Transformation|GetActorForwardVector _returnvalue) 1e+02))))

(fn OwnerUseItem
  (params (ItemID :type Name) (Index :type Integer) (Quantity :type Integer))
  (bind _returnvalue (Utilities|GetDataTableRow "/Game/Blueprints/Items/DT_ItemData.DT_ItemData" ItemID)
    (:then
      (switch Utilities|FlowControl|Switch|SwitchonE_ItemType (.ItemType (Utilities|Struct|BreakF_ItemStruct _returnvalue))
        (:NewEnumerator0
          (Math|Integer|DecrementInt Quantity
            (:%20%20
              (bind _asbp_unit_base (Utilities|Casting|CastToBP_UnitBase (Components|GetOwner)))
              (Default|Interacting _asbp_unit_base 0.0)
              (CallFunction|RemovefromInventory Index true 1))))
        (:NewEnumerator1
          (bind _asbp_unit_base_2 (Utilities|Casting|CastToBP_UnitBase (Components|GetOwner)))
          (Utilities|IsValid (Variables|/Game/Blueprints/Units/UnitBlueprints/BP_UnitBase.BP_UnitBase_C|GetEquippedWeapon _asbp_unit_base_2)
            (:Is%20Valid
              (if (== (Utilities|GetClass (Variables|/Game/Blueprints/Units/UnitBlueprints/BP_UnitBase.BP_UnitBase_C|GetEquippedWeapon _asbp_unit_base_2)) (.ItemClass (Utilities|Struct|BreakF_ItemStruct _returnvalue)))
                (Actor|DestroyActor (Variables|/Game/Blueprints/Units/UnitBlueprints/BP_UnitBase.BP_UnitBase_C|GetEquippedWeapon _asbp_unit_base_2))
                (else
                  (Actor|DestroyActor (Variables|/Game/Blueprints/Units/UnitBlueprints/BP_UnitBase.BP_UnitBase_C|GetEquippedWeapon _asbp_unit_base_2))
                  (bind _returnvalue_2 (Game|SpawnActorfromClass (.ItemClass (Utilities|Struct|BreakF_ItemStruct _returnvalue)) (Math|Transform|MakeTransform (.location (Transformation|GetActorTransform _asbp_unit_base_2)) (.rotation (Transformation|GetActorTransform _asbp_unit_base_2)) "1.000000,1.000000,1.000000") "Undefined" "MultiplyWithRoot" 0 0 :!label _label))
                  (Variables|/Game/Blueprints/Inventory/BP_ItemDataComponent.BP_ItemDataComponent_C|SetAmmo (Variables|/Game/Blueprints/Items/Weapons/BP_WeaponBase.BP_WeaponBase_C|GetBP_ItemDataComponent (.AsBP%20Weapon%20Base (Utilities|Casting|CastToBP_WeaponBase _returnvalue_2))) (.Ammo (Utilities|Struct|BreakF_SlotStruct (Utilities|Array|Get(acopy) (Variables|Default|GetContents) Index))))
                  (Default|EquipItem _asbp_unit_base_2 (.AsBP%20Weapon%20Base (Utilities|Casting|CastToBP_WeaponBase _returnvalue_2))))))
            (:Is%20Not%20Valid
              (goto _label))))))))

(fn FindSpecificContents
  (params (ItemID :type Name))
  (bind _local_firstindex (LocalVariables|GetLocal_FirstIndex))
  (Utilities|Array|Clear _local_firstindex)
  (LocalVariables|SetLocal_TotalCount 0)
  (for (_array_element _array_index) (Variables|Default|GetContents)
    (if (== ItemID (.ItemID (Utilities|Struct|BreakF_SlotStruct _array_element)))
      (Utilities|Array|AddUnique _local_firstindex _array_index)
      (LocalVariables|SetLocal_TotalCount (+ (.Quantity (Utilities|Struct|BreakF_SlotStruct _array_element)) (LocalVariables|GetLocal_TotalCount)))))
  (return (LocalVariables|GetLocal_FirstIndex) (LocalVariables|GetLocal_TotalCount)))

(fn HasWeapon
  (for (_array_element _array_index) (Variables|Default|GetContents)
    (bind _returnvalue (Utilities|GetDataTableRow "/Game/Blueprints/Items/DT_ItemData.DT_ItemData" (.ItemID (Utilities|Struct|BreakF_SlotStruct _array_element)))
      (:then
        (if (Utilities|Enum|Equal(Enum) (.ItemType (Utilities|Struct|BreakF_ItemStruct _returnvalue)) "NewEnumerator1")
          (return (.ItemID (Utilities|Struct|BreakF_SlotStruct _array_element)) _array_index)))))
  (return "None" -1))

(fn Lookat
  (return))