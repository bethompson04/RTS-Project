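; Item data component that makes its owning actor a pickup which units can collect into their inventory.
; On interaction, it passes its item row name, quantity and ammo to the unit's BPInventoryComponent, skipping weapons that are already equipped.
; A successful add stores the inventory index, destroys the owner and has RTS player 0 update its inventory.
; LookAt is an empty stub.
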(event EventBeginPlay)

(event EventTick
  (params (DeltaSeconds :type Float%20%28single-precision%29)))

(event EventInteractwith
  (params (InteractingUnit :type BP%20Unit%20Base%20Object%20Reference))
  (bind _bp_inventorycomponent (Variables|/Game/Blueprints/Units/UnitBlueprints/BP_UnitBase.BP_UnitBase_C|GetBP_InventoryComponent InteractingUnit))
  (bind _asbp_weapon_base (Utilities|Casting|CastToBP_WeaponBase (Components|GetOwner))
    (:then
      (if (not (Variables|/Game/Blueprints/Items/Weapons/BP_WeaponBase.BP_WeaponBase_C|GetEquipped _asbp_weapon_base))
        (Utilities|IsValid _bp_inventorycomponent :!label _label
          (:Is%20Valid
            (bind (_success _quantityremaining _index) (Default|AddtoInventory _bp_inventorycomponent (.rowname (Variables|Default|GetItemID)) (Variables|Default|GetQuantity) (Variables|Default|GetAmmo)))
            (if _success
              (Variables|Default|SetInventoryIndex _index)
              (Actor|DestroyActor (Components|GetOwner))
              (Default|UpdateInventory (CallFunction|GetRTSPlayer) false))))))
    (:CastFailed
      (goto _label))))

(fn Lookat
  (return))