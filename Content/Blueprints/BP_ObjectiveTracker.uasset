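; BP_ObjectiveTracker runs a mission's queue of objectives: Extermination, VIP Evac and Interact.
; It binds completion events for the front objective; Extermination counts non-team-1 units down, Interact completes immediately on interaction, and VIP Evac's handler is empty.
; Completed objectives leave the array, and an empty queue saves player units and shows the mission-completed widget.
; It also offers a mission-failed screen and a nearest-enemy-squad lookup.
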(event Custom|UpdateObjective
  (params (ObjectiveCount :type Integer))
  (if (<= (Variables|Default|GetEnemies%20Remaining) 0)
    (Variables|Default|SetObjectiveStatus true))
  (if (not (Variables|Default|GetObjectiveStatus))
    (switch Utilities|FlowControl|Switch|SwitchonE_MissionType (.ObjectiveType (Utilities|Struct|BreakF_ObjectiveStruct (Utilities|Array|Get(acopy) (Variables|Default|GetObjectiveType))))
      (:NewEnumerator1
        (Development|PrintText (Utilities|Text|FormatText "Enemies Remaining: {EnemyCount}" ObjectiveCount)))
      (:NewEnumerator0
        (Development|PrintText (Utilities|Text|FormatText "VIP's Remaining: {VIPCount}" ObjectiveCount)))
      (:NewEnumerator3
        (Development|PrintText (Utilities|Text|FormatText "INTERACT"))))
    (else
      (CallFunction|ObjectiveComplete))))

(event Custom|AllObjectivesComplete
  (Utilities|FlowControl|Delay 5.0)
  (bind _playerunitsave (Default|GetPlayerSave (CallFunction|GetRTSPlayer)))
  (Class|BPISaveGame|SavePlayerUnits(Message) (Game|GetGameInstance) _playerunitsave false)
  (bind _returnvalue (UserInterface|CreateWidget "/Game/Blueprints/UserInterface/Menus/WBP_MissionCompleted.WBP_MissionCompleted_C"))
  (UserInterface|Viewport|AddtoViewport _returnvalue 0))

(event Custom|MissionFailed
  (bind _returnvalue (UserInterface|CreateWidget "/Game/Blueprints/UserInterface/Menus/WBP_MissionFailed.WBP_MissionFailed_C"))
  (UserInterface|Viewport|AddtoViewport _returnvalue 0))

(event Custom|CheckUnitAffiliation
  (params (UnitTeam :type Integer))
  (if (!= UnitTeam 1)
    (bind _result (Math|Integer|DecrementInt (Variables|Default|GetEnemies%20Remaining))
      (:%20%20
        (bind _output_get (Variables|Default|SetEnemies%20Remaining _result))
        (CallFunction|UpdateObjective _output_get)))))

(event Custom|VIPEvac)

(event Custom|ObjectiveComplete
  (bind _objectivetype (Variables|Default|GetObjectiveType))
  (Utilities|Array|RemoveIndex _objectivetype)
  (if (> (Utilities|Array|Length _objectivetype) 0)
    (Variables|Default|SetObjectiveStatus false)
    (CallFunction|BeginObjective)
    (else
      (CallFunction|AllObjectivesComplete))))

(event Custom|BeginObjective
  (Variables|Default|SetEnemies%20Remaining 0)
  (Variables|Default|SetVIPs%20to%20Escort 0)
  (Utilities|FlowControl|Delay 1.0)
  (CallFunction|InitObjective)
  (switch Utilities|FlowControl|Switch|SwitchonE_MissionType (.ObjectiveType (Utilities|Struct|BreakF_ObjectiveStruct (Utilities|Array|Get(acopy) (Variables|Default|GetObjectiveType))))
    (:NewEnumerator1
      (EventDispatchers|BindEventtoUnitKilled (delegate Custom|CheckUnitAffiliation)))
    (:NewEnumerator0
      (EventDispatchers|BindEventtoVIPEvacuated (delegate Custom|VIPEvac)))
    (:NewEnumerator3
      (EventDispatchers|BindEventtoObjectiveInteractedwith (delegate Custom|Interacted)))))

(event Custom|Interacted
  (params (Objective :type Actor%20Object%20Reference))
  (Variables|Default|SetObjectiveStatus true)
  (CallFunction|ObjectiveComplete))

(event EventBeginPlay
  (CallFunction|BeginObjective))

(event EventTick
  (params (DeltaSeconds :type Float%20%28single-precision%29)))

(fn ConstructionScript)

(fn InitObjective
  (switch Utilities|FlowControl|Switch|SwitchonE_MissionType (.ObjectiveType (Utilities|Struct|BreakF_ObjectiveStruct (Utilities|Array|Get(acopy) (Variables|Default|GetObjectiveType))))
    (:NewEnumerator1
      (Development|PrintString "Kill all enemies")
      (bind _outactors (Actor|GetAllActorsOfClass "/Game/Blueprints/Units/UnitBlueprints/BP_UnitBase.BP_UnitBase_C"))
      (for _array_element _outactors
        (bind _teamid (Default|GetTeam _array_element))
        (if (!= _teamid 1)
          (bind _result (Math|Integer|IncrementInt (Variables|Default|GetEnemies%20Remaining))
            (:%20%20
              (Variables|Default|SetEnemies%20Remaining _result)))))
      (Development|PrintString (Utilities|String|ToString(Integer) (Variables|Default|GetEnemies%20Remaining))))
    (:NewEnumerator0
      (Development|PrintString "Extract VIPs"))))

(fn GetClosestObjective
  (params (InActor :type Actor%20Object%20Reference))
  (bind _teamid (Class|IBPRTS|GetTeam(Message) InActor))
  (switch Utilities|FlowControl|Switch|SwitchonE_MissionType (.ObjectiveType (Utilities|Struct|BreakF_ObjectiveStruct (Utilities|Array|Get(acopy) (Variables|Default|GetObjectiveType))))
    (:NewEnumerator1
      _)
    (:NewEnumerator3
      _))
  (bind _outactors (Actor|GetAllActorsOfClass "/Game/Blueprints/Units/BP_Squad.BP_Squad_C"))
  (for _array_element _outactors
    (bind _teamid_2 (Class|IBPRTS|GetTeam(Message) (Variables|/Game/Blueprints/Units/BP_Squad.BP_Squad_C|GetSquadLeader _array_element)))
    (if (and (!= _teamid_2 0) (!= _teamid_2 _teamid))
      (if (or (< (Transformation|GetDistanceTo InActor _array_element) (LocalVariables|GetLocalClosestDistance)) (== (LocalVariables|GetLocalClosestDistance) -1.0))
        (LocalVariables|SetLocalClosestDistance (Transformation|GetDistanceTo InActor _array_element))
        (LocalVariables|SetLocalClosestObjective _array_element))))
  (return (LocalVariables|GetLocalClosestObjective)))

(fn GetGameData
  (return 0))