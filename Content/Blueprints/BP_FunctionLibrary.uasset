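; Blueprint function library of shared helpers for an RTS game.
; It fetches the RTS player controller by player index and returns the squad leader of a player's selected squad, with validity checks.
; A camera helper finds the RTS camera actor by class and moves it straight to a given location.
; UseItem is an empty stub.
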(fn GetPlayerSquadLeader
  (params (Player :type BP%20RTS%20Player%20Controller%20Object%20Reference))
  (bind _selectedsquad (Variables|/Game/Blueprints/BP_RTSPlayerController.BP_RTSPlayerController_C|GetSelectedSquad Player))
  (bind _squadleader (Variables|/Game/Blueprints/Units/BP_Squad.BP_Squad_C|GetSquadLeader _selectedsquad))
  (Utilities|IsValid _selectedsquad
    (:Is%20Valid
      (Utilities|IsValid _squadleader
        (:Is%20Valid
          (return _squadleader))
        (:Is%20Not%20Valid
          _)))
    (:Is%20Not%20Valid
      _))
  (return 0))

(fn GetRTSPlayer
  (params (PlayerIndex :type Integer))
  (bind _asbp_rtsplayer_controller (Utilities|Casting|CastToBP_RTSPlayerController (Game|GetPlayerController 0 PlayerIndex))
    (:then
      (return _asbp_rtsplayer_controller))
    (:CastFailed
      (return 0))))

(fn UseItem
  (params (UseTime :type Float%20%28double-precision%29)))

(fn FocusCamerato
  (params (FocusLocation :type Vector))
  (bind _returnvalue (Actor|GetActorOfClass 0 "/Game/Blueprints/BP_RTSPlayerCamera.BP_RTSPlayerCamera_C"))
  (Transformation|SetActorLocation _returnvalue FocusLocation false false))