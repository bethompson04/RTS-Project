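; Player HUD that provides drag-box unit selection for an RTS.
; Pressed, Held and Released events track the mouse start and current positions and toggle drawing of a translucent rectangle.
; While dragging, DrawHUD rebuilds the RTS player controller's SelectedUnits every frame from units inside the rectangle, calling SelectedMessage on each.
; The selection query runs inside DrawHUD, as GetActorsInSelectionRectangle requires.
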(event EventPressed
  (bind _returnvalue (Game|GetPlayerController 0))
  (bind (_locationx _locationy) (Game|Player|GetMousePosition _returnvalue))
  (Variables|Default|SetSelectionBoxDraw true)
  (bind _output_get (Variables|Default|SetMouseStart (Math|Vector2D|MakeVector2D _locationx _locationy)))
  (Variables|Default|SetMouseCurrent _output_get))

(event EventHeld
  (bind _returnvalue (Game|GetPlayerController 0))
  (bind (_locationx _locationy) (Game|Player|GetMousePosition _returnvalue))
  (Variables|Default|SetMouseCurrent (Math|Vector2D|MakeVector2D _locationx _locationy)))

(event EventReleased
  (Variables|Default|SetSelectionBoxDraw false))

(event EventDrawHUD
  (params (SizeX :type Integer) (SizeY :type Integer))
  (bind _mousestart (Variables|Default|GetMouseStart))
  (bind _mousecurrent (Variables|Default|GetMouseCurrent))
  (if (Variables|Default|GetSelectionBoxDraw)
    (HUD|DrawRect "(R=0.000000,G=0.735736,B=1.000000,A=0.200000)" (.x _mousestart) (.y _mousestart) (- (.x _mousecurrent) (.x _mousestart)) (- (.y _mousecurrent) (.y _mousestart)))
    (bind _asbp_rtsplayer_controller (Utilities|Casting|CastToBP_RTSPlayerController (Game|GetPlayerController 0)))
    (Utilities|Array|Clear (Variables|/Game/Blueprints/BP_RTSPlayerController.BP_RTSPlayerController_C|GetSelectedUnits _asbp_rtsplayer_controller))
    (for _array_element (Class|HUD|GetActorsinSelectionRectangle "/Game/Blueprints/Units/BP_UnitBase.BP_UnitBase_C" (Variables|Default|GetMouseStart) (Variables|Default|GetMouseCurrent) false false)
      (Class|IBPRTS|Selected(Message) _array_element)
      (bind _asbp_unit_base (Utilities|Casting|CastToBP_UnitBase _array_element))
      (Utilities|Array|AddUnique (Variables|/Game/Blueprints/BP_RTSPlayerController.BP_RTSPlayerController_C|GetSelectedUnits _asbp_rtsplayer_controller) _asbp_unit_base))))

(fn ConstructionScript)