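; HUD for an RTS that draws a mouse-drag selection box and turns the boxed units into the player's selected squad.
; Pressed, Held and Released events track the box corners, and DrawHUD queries BP_UnitBase actors inside it every frame while dragging.
; A DoOnce, reset between drags, adopts the first unit's squad on the RTS player controller, then boxed units join it.
; The squad then updates its leader and selected message, while an empty box sends a deselect message.
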(event EventPressed
  (bind _returnvalue (Game|GetPlayerController 0))
  (bind (_locationx _locationy) (Game|Player|GetMousePosition _returnvalue))
  (Variables|Default|SetSelectionBoxDraw true)
  (bind _output_get (Variables|Default|SetMouseStart (Math|Vector2D|MakeVector2D _locationx _locationy)))
  (Variables|Default|SetMouseCurrent _output_get))

(event EventHeld
  (bind _returnvalue (Game|GetPlayerController 0))
  (bind (_locationx _locationy) (Game|Player|GetMousePosition _returnvalue))
  (Variables|Default|SetMouseCurrent (Math|Vector2D|MakeVector2D _locationx _locationy)))

(event EventReleased
  (Variables|Default|SetSelectionBoxDraw false))

(event EventDrawHUD
  (params (SizeX :type Integer) (SizeY :type Integer))
  (bind _mousestart (Variables|Default|GetMouseStart))
  (bind _mousecurrent (Variables|Default|GetMouseCurrent))
  (bind _mousestart_2 (Variables|Default|GetMouseStart))
  (bind _mousecurrent_2 (Variables|Default|GetMouseCurrent))
  (bind _outactors (Class|HUD|GetActorsinSelectionRectangle "/Game/Blueprints/Units/BP_UnitBase.BP_UnitBase_C" _mousestart _mousecurrent false false))
  (if (Variables|Default|GetSelectionBoxDraw)
    (HUD|DrawRect "(R=0.000000,G=0.735736,B=1.000000,A=0.200000)" (.x _mousestart_2) (.y _mousestart_2) (- (.x _mousecurrent_2) (.x _mousestart_2)) (- (.y _mousecurrent_2) (.y _mousestart_2)))
    (bind _asbp_rtsplayer_controller (Utilities|Casting|CastToBP_RTSPlayerController (Game|GetPlayerController 0)))
    (Utilities|IsValid (Variables|/Game/Blueprints/BP_RTSPlayerController.BP_RTSPlayerController_C|GetSelectedSquad _asbp_rtsplayer_controller)
      (:Is%20Valid
        _)
      (:Is%20Not%20Valid
        _))
    (if (Utilities|Array|IsNotEmpty _outactors) ; False if box empty
      (for _array_element _outactors
        (bind _asbp_unit_base (Utilities|Casting|CastToBP_UnitBase _array_element))
        (Utilities|FlowControl|Sequence
          (:then_0
            (Utilities|FlowControl|DoOnce false
              (:Completed
                (bind _output_get (Variables|/Game/Blueprints/BP_RTSPlayerController.BP_RTSPlayerController_C|SetSelectedSquad _asbp_rtsplayer_controller (Variables|/Game/Blueprints/Units/BP_UnitBase.BP_UnitBase_C|GetSquad _asbp_unit_base))))))
          (:then_1
            (if (not (and (!= _output_get (Variables|/Game/Blueprints/Units/BP_UnitBase.BP_UnitBase_C|GetSquad _asbp_unit_base)) (Utilities|Array|ContainsItem (Variables|/Game/Blueprints/Units/BP_Squad.BP_Squad_C|GetSquadMembers (Variables|/Game/Blueprints/BP_RTSPlayerController.BP_RTSPlayerController_C|GetSelectedSquad _asbp_rtsplayer_controller)) _asbp_unit_base))) ; If the selected squad has unit
              (Default|AddtoSquad _output_get _asbp_unit_base)))))
      (Default|SetLeader (Variables|/Game/Blueprints/BP_RTSPlayerController.BP_RTSPlayerController_C|GetSelectedSquad _asbp_rtsplayer_controller))
      (Class|IBPRTS|Selected(Message) (Variables|/Game/Blueprints/BP_RTSPlayerController.BP_RTSPlayerController_C|GetSelectedSquad _asbp_rtsplayer_controller))
      (else
        (Utilities|IsValid (Variables|/Game/Blueprints/BP_RTSPlayerController.BP_RTSPlayerController_C|GetSelectedSquad _asbp_rtsplayer_controller)
          (:Is%20Valid
            (Class|IBPRTS|Deselected(Message) (Variables|/Game/Blueprints/BP_RTSPlayerController.BP_RTSPlayerController_C|GetSelectedSquad _asbp_rtsplayer_controller))))))
    (else
      (Utilities|FlowControl|DoOnce false) ; enters at Reset
    )))

(fn ConstructionScript)